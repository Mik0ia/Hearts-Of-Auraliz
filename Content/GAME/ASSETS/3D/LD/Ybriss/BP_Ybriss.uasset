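; Ybriss actor that swings two scene components back and forth in opposite yaw, starting at BeginPlay.
; MoveBack and MoveFront hand off to each other near ±10 degrees of yaw, using timelines as per-frame tickers with fixed increments and DoOnce gates against re-entry.
; A separate Play event, not called in this graph, loops a timeline that adds its track value to actor Z each update.
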(event Custom|MoveBack
  (bind _scene (Variables|Default|GetScene))
  (bind _scene1 (Variables|Default|GetScene1))
  (bind _relativerotation (Variables|/Script/Engine.SceneComponent|GetRelativeRotation _scene1))
  (bind _relativerotation_2 (Variables|/Script/Engine.SceneComponent|GetRelativeRotation _scene))
  (bind _returnvalue (+ (.yaw _relativerotation_2) 0.2))
  (Utilities|FlowControl|DoOnce false :!label _label
    (:Completed
      (Timeline|Timeline_0 PlayFromStart
        (:Update
          (if (>= _returnvalue 1e+01)
            (CallFunction|MoveFront)
            (Utilities|FlowControl|Sequence
              (:then_0
                (Timeline|Timeline_0 Stop))
              (:then_1
                (goto _label Reset)))
            (else
              (Transformation|SetRelativeRotation _scene (Math|Rotator|MakeRotator (.roll _relativerotation_2) (.pitch _relativerotation_2) _returnvalue) false false)
              (Transformation|SetRelativeRotation (Variables|Default|GetScene1) (Math|Rotator|MakeRotator (.roll _relativerotation) (.pitch _relativerotation) (+ (.yaw _relativerotation) -0.2)) false false))))))))

(event Custom|Play
  (bind _returnvalue (Transformation|GetActorLocation))
  (bind _newtrack_0 (Timeline|Timeline PlayFromStart)
    (:Update
      (Transformation|SetActorLocation (Math|Vector|MakeVector (.x _returnvalue) (.y _returnvalue) (+ _newtrack_0 (.z _returnvalue))) false false))
    (:Finished
      (CallFunction|Play))))

(event Custom|MoveFront
  (bind _scene (Variables|Default|GetScene))
  (bind _scene1 (Variables|Default|GetScene1))
  (bind _relativerotation (Variables|/Script/Engine.SceneComponent|GetRelativeRotation _scene))
  (bind _relativerotation_2 (Variables|/Script/Engine.SceneComponent|GetRelativeRotation _scene1))
  (bind _returnvalue (+ (.yaw _relativerotation) -0.2))
  (Utilities|FlowControl|DoOnce false :!label _label
    (:Completed
      (Timeline|Timeline_1 PlayFromStart
        (:Update
          (if (<= _returnvalue -1e+01)
            (CallFunction|MoveBack)
            (Utilities|FlowControl|Sequence
              (:then_0
                (Timeline|Timeline_1 Stop))
              (:then_1
                (goto _label Reset)))
            (else
              (Transformation|SetRelativeRotation _scene (Math|Rotator|MakeRotator (.roll _relativerotation) (.pitch _relativerotation) _returnvalue) false false)
              (Transformation|SetRelativeRotation (Variables|Default|GetScene1) (Math|Rotator|MakeRotator (.roll _relativerotation_2) (.pitch _relativerotation_2) (+ (.yaw _relativerotation_2) 0.2)) false false))))))))

(event EventBeginPlay
  (CallFunction|MoveBack))

(event Collision|EventActorBeginOverlap
  (params (OtherActor :type Actor%20Object%20Reference)))

(fn ConstructionScript)