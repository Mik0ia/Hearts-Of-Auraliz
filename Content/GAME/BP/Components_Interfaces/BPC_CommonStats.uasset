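; BPC_CommonStats is a component that provides a battle speed stat shared by player and enemy characters.
; On BeginPlay it finds and caches the GM_BattleGameMode through an actor search.
; GetSpeed branches on IsEnnemy and asks the game mode for the buffed stat, passing either the enemy's battle component or the player's playable character component.
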(event EventBeginPlay
  (bind _outactors (Actor|GetAllActorsOfClass "/Game/GAME/BP/General/GM_BattleGameMode.GM_BattleGameMode_C"))
  (Variables|Default|SetGM_Battle (Utilities|Array|Get(acopy) _outactors)))

(fn GetSpeed
  (bind _gm_battle (Variables|Default|GetGM_Battle))
  (if (Variables|Default|GetIsEnnemy?)
    (return (Default|GetStat+Buff _gm_battle "NewEnumerator4" (Variables|/Game/GAME/BP/InBattle/Ennemy/BP_BasicWildEnnemy.BP_BasicWildEnnemy_C|GetBPC_CharacterBattleComponent (Variables|Default|GetBP_Ennemy)) 0 true))
    (else
      (return (Default|GetStat+Buff _gm_battle "NewEnumerator4" 0 (Variables|/Game/GAME/BP/InBattle/Manieur_Armes/BP_PlayableCharacterInBattle.BP_PlayableCharacterInBattle_C|GetBPC_PlayableCharacter (Variables|Default|GetBP_Player)) false)))))