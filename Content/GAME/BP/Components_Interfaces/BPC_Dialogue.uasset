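; Dialogue component that runs branching, DataTable-driven conversations in a WBP_Dialogue widget and flags the player as in dialogue.
; Rows are looked up by index, advancing through NextRow or the chosen option's index until -1 closes the widget with a reversed Open animation.
; On advancing, a row's effects can launch battles, give items, increase Echo or fire scripted GameMode story and camera events through a large enum switch.
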(event Custom|LaunchDialogue
  (params (Data%20Table :type Data%20Table%20Object%20Reference) (Index :type Integer))
  (Variables|Default|SetCurrentRowIndex Index)
  (Variables|Default|SetDialogueDataTable Data%20Table)
  (CallFunction|CreateWidget)
  (CallFunction|ShowDialogue Data%20Table Index))

(event Custom|NextDialogue
  (params (Row :type Integer))
  (bind _returnvalue (Utilities|GetDataTableRow (Variables|Default|GetDialogueDataTable) (Utilities|String|StringToName (Utilities|String|ToString(Integer) Row)))
    (:then
      (if (not (Utilities|Array|IsEmpty (.DialogueEffectEnum (Utilities|Struct|BreakST_Dialogue _returnvalue))))
        (for (_array_element _array_index) (.DialogueEffectEnum (Utilities|Struct|BreakST_Dialogue _returnvalue))
          (CallFunction|DoDialogueEffect _array_element (Utilities|Array|Get(acopy) (.DialogueEffect (Utilities|Struct|BreakST_Dialogue _returnvalue)) _array_index))))
      (if (not (.IsChoice? (Utilities|Struct|BreakST_Dialogue _returnvalue)))
        (if (== (.NextRow (Utilities|Struct|BreakST_Dialogue _returnvalue)) -1)
          (CallFunction|CloseDialogue (.LastRowIndex (Utilities|Struct|BreakST_Dialogue _returnvalue)))
          (else
            (bind _output_get (Variables|Default|SetCurrentRowIndex (.NextRow (Utilities|Struct|BreakST_Dialogue _returnvalue))))
            (CallFunction|ShowDialogue (Variables|Default|GetDialogueDataTable) _output_get)))))))

(event Custom|CloseDialogue
  (params (LastRowIndex :type Integer))
  (bind _wbp_dialogue (Variables|Default|GetWBP_Dialogue))
  (Default|CallFinishedDialogue)
  (Variables|Default|SetCurrentRowIndex LastRowIndex)
  (Components|Animation|PlayAnimation _wbp_dialogue (Variables|/Game/GAME/BP/Widget/WBP_Dialogue.WBP_Dialogue_C|GetOpen _wbp_dialogue) 0.0 1 "Reverse"
    (:Finished
      (Default|SetIsinDialogueStatus (Variables|Default|GetPlayer) false self)
      (Widget|RemovefromParent _wbp_dialogue))))

(event Custom|ShowDialogue
  (params (DataTable :type Data%20Table%20Object%20Reference) (Index :type Integer))
  (bind _returnvalue (Utilities|GetDataTableRow DataTable (Utilities|String|StringToName (Utilities|String|ToString(Integer) Index)))
    (:then
      (Default|SetVisuals (Variables|Default|GetWBP_Dialogue) self _returnvalue)
      (Default|SetIsinDialogueStatus (Variables|Default|GetPlayer) true self))
    (:RowNotFound
      (Development|PrintString "dialogue pas trouvé"))))

(event Custom|CreateWidget
  (bind _returnvalue (UserInterface|CreateWidget "/Game/GAME/BP/Widget/WBP_Dialogue.WBP_Dialogue_C"))
  (Variables|Default|SetWBP_Dialogue _returnvalue)
  (UserInterface|Viewport|AddtoViewport _returnvalue 0)
  (Class|UserWidget|PlayAnimationForward (Variables|Default|GetWBP_Dialogue) (Variables|/Game/GAME/BP/Widget/WBP_Dialogue.WBP_Dialogue_C|GetOpen (Variables|Default|GetWBP_Dialogue)) 1.0 false))

(event Custom|ValidateChoice
  (params (ChoiceIndex :type Integer))
  (Audio|PlaySound2D "/Game/GAME/AUDIO/SE/BattleMenu/Button_Pressed.Button_Pressed" 1.0 1.0 0.0 0 0)
  (Default|HideAllChoice (Variables|Default|GetWBP_Dialogue))
  (Variables|Default|SetIsInChoice? false)
  (Variables|Default|SetCanSkip? false)
  (bind _output_get (Variables|Default|SetCurrentRowIndex (Utilities|Array|Get(acopy) (Variables|Default|GetCurrentChoiceNextIndex) ChoiceIndex)))
  (CallFunction|ShowDialogue (Variables|Default|GetDialogueDataTable) _output_get))

(fn DoDialogueEffect
  (params (Effect :type E_DialogueEffect%20Enum :default "NewEnumerator0") (Structure :type ST%20Dialogue%20Effect%20Structure))
  (bind (_battletable _battleindex _itemtogain _eventtocast _echotoincreasevalue _echoindex) (Utilities|Struct|BreakST_DialogueEffect Structure))
  (bind _player (Variables|Default|GetPlayer))
  (bind _gm_ref (Variables|/Game/GAME/BP/Overworld/BP_PlayerCharacter.BP_PlayerCharacter_C|GetGM%20Ref _player))
  (switch Utilities|FlowControl|Switch|SwitchonE_DialogueEffect Effect
    (:NewEnumerator0
      (Default|LaunchBattle (Variables|Default|GetPlayer) _battleindex _battletable))
    (:NewEnumerator2
      (for _array_element _itemtogain
        (Default|GetItem (Variables|/Game/GAME/BP/General/GM_OverworldGameMode.GM_OverworldGameMode_C|GetAs%20GI%20Game%20Instance _gm_ref) _array_element)))
    (:NewEnumerator3
      (switch Utilities|FlowControl|Switch|SwitchonE_GamemodeEvent _eventtocast
        (:NewEnumerator0
          (Default|LizEnters _gm_ref))
        (:NewEnumerator1
          (Default|OndeFalls _gm_ref))
        (:NewEnumerator2
          (Default|OndeGetUp _gm_ref))
        (:NewEnumerator3
          (Default|LizLeaving _gm_ref))
        (:NewEnumerator4
          (Default|FinishIntro _gm_ref))
        (:NewEnumerator5
          (Default|OndeApproaching _gm_ref))
        (:NewEnumerator6
          (Default|Ondefocus _gm_ref))
        (:NewEnumerator8
          (Default|KentoFocus _gm_ref))
        (:NewEnumerator10
          (Default|OndeShocked _gm_ref))
        (:NewEnumerator11
          (Default|OndeNotShocked _gm_ref))
        (:NewEnumerator12
          (Default|PouloieEvent _gm_ref))
        (:NewEnumerator13
          (Default|PouloieExit _gm_ref))
        (:NewEnumerator14
          (Default|GoFacePouloie _gm_ref))
        (:NewEnumerator15
          (Default|PouloieLeaving _gm_ref))
        (:NewEnumerator16
          (Default|PouloieCam _gm_ref))
        (:NewEnumerator17
          (Default|KentoFinishedEvent _gm_ref))
        (:NewEnumerator18
          (Default|PouloieBattleFrontCam _gm_ref))
        (:NewEnumerator19
          (Default|FrontOndeBattle _gm_ref))
        (:NewEnumerator20
          (Default|GiganticBoom _gm_ref))
        (:NewEnumerator21
          (Default|OndeTurnAround _gm_ref))
        (:NewEnumerator22
          (Default|ExitPouloieSolo _gm_ref))
        (:NewEnumerator23
          (Default|FocusKentoBattle _gm_ref))
        (:NewEnumerator24
          (Default|FocusAshkar _gm_ref))
        (:NewEnumerator25
          (Default|LargeBattleCam _gm_ref))
        (:NewEnumerator26
          (Default|FocusOndeAbordage _gm_ref))
        (:NewEnumerator27
          (Default|AshkarAttack _gm_ref))
        (:NewEnumerator28
          (Default|RemoveFadeEvent _gm_ref))
        (:NewEnumerator29
          (Default|EgoCam _gm_ref))
        (:NewEnumerator30
          (Default|OndeCamShockedIntroIsland _gm_ref))
        (:NewEnumerator31
          (Default|SimpleOndeIslandIntroFocus _gm_ref))
        (:NewEnumerator32
          (Default|EgoStandUp _gm_ref))
        (:NewEnumerator33
          (Default|EgoLeaving _gm_ref))
        (:NewEnumerator34
          (Default|EgoCorabeFocus _gm_ref))
        (:NewEnumerator35
          (Default|OndeCorabeFocus _gm_ref))
        (:NewEnumerator36
          (Default|LargeCorabeCam _gm_ref))
        (:NewEnumerator37
          (Default|OtherCorabeEvent _gm_ref))
        (:NewEnumerator39
          (Default|OpeningCorabeEvent _gm_ref))
        (:NewEnumerator40
          (Default|OndeSwordCorabeFocus _gm_ref))
        (:NewEnumerator41
          (Default|EgoSwordCorabe _gm_ref))
        (:NewEnumerator42
          (Default|EndCorabeBeatenEvent _gm_ref))
        (:NewEnumerator44
          (Default|FireCampEvent _gm_ref))
        (:NewEnumerator45
          (Default|GoBackRoad _gm_ref))))
    (:NewEnumerator5
      (Default|IncreaseEcho (Variables|/Game/GAME/BP/General/GM_OverworldGameMode.GM_OverworldGameMode_C|GetAs%20GI%20Game%20Instance (Variables|/Game/GAME/BP/Overworld/BP_PlayerCharacter.BP_PlayerCharacter_C|GetGM%20Ref (Variables|Default|GetPlayer))) _echotoincreasevalue _echoindex))))