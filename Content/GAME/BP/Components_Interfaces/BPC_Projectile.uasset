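; Battle projectile component that resolves a hit between a playable character and a wild enemy, bound to HitEnnemy at BeginPlay.
; Enemy hits check the battle pawn's defence state: parry triggers PARRYEVENT, half-raised guard damages both character and linked AllyArmeManieur, full guard redirects damage to that ally.
; Player hits calculate damage from buffed stats, level and elements through GMBattle, then handle kills, victory or turn end.
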(event Custom|HitEnnemy_Event
  (bind _bpc_target (Variables|Default|GetBPC_Target))
  (bind _move_infos (Variables|Default|GetMove_Infos))
  (bind _bpc_attacker (Variables|Default|GetBPC_Attacker))
  (bind _move (Variables|Default|GetMove))
  (bind _gm_battle (Variables|/Game/GAME/BP/Components_Interfaces/BPC_CommonStats.BPC_CommonStats_C|GetGM_Battle _bpc_target))
  (bind _gm_battle_2 (Variables|/Game/GAME/BP/Components_Interfaces/BPC_CommonStats.BPC_CommonStats_C|GetGM_Battle _bpc_attacker))
  (bind _bp_inbattlepawn (Variables|/Game/GAME/BP/General/GM_BattleGameMode.GM_BattleGameMode_C|GetBp_InBattlePawn _gm_battle))
  (bind _bp_inbattlepawn_2 (Variables|/Game/GAME/BP/General/GM_BattleGameMode.GM_BattleGameMode_C|GetBp_InBattlePawn _gm_battle_2))
  (bind _asbp_playable_character_in_battle (Utilities|Casting|CastToBP_PlayableCharacterInBattle (Components|GetOwner _bpc_target))
    (:then
      (Development|PrintString (Utilities|String|Append (Utilities|GetDisplayName _asbp_playable_character_in_battle) " : " "cible projectile") true true "(R=1.000000,G=0.976883,B=0.000000,A=1.000000)")
      (bind _asbp_basic_wild_ennemy (Utilities|Casting|CastToBP_BasicWildEnnemy (Components|GetOwner (Variables|Default|GetBPC_Attacker))))
      (Utilities|FlowControl|DoOnce false
        (:Completed
          (if (Variables|/Game/GAME/BP/InBattle/BP_InBattlePawn.BP_InBattlePawn_C|GetPARRY _bp_inbattlepawn)
            (Default|PARRYEVENT _bp_inbattlepawn (Transformation|GetWorldLocation (Variables|/Game/GAME/BP/InBattle/Manieur_Armes/BP_PlayableCharacterInBattle.BP_PlayableCharacterInBattle_C|GetSkeletalMesh _asbp_playable_character_in_battle)) "NewEnumerator0")
            (Default|EndMyTurn _asbp_basic_wild_ennemy :!label _label)
            (elif (Variables|/Game/GAME/BP/InBattle/BP_InBattlePawn.BP_InBattlePawn_C|GetIsPuttingGuardUp? _bp_inbattlepawn)
              (Development|PrintString "DOUBLE DAMAGE" true true "(R=1.000000,G=0.000000,B=0.037576,A=1.000000)")
              (bind (_damage _is_effective_) (Default|CalcDamage _asbp_basic_wild_ennemy _asbp_playable_character_in_battle _move false))
              (Development|PrintString (Utilities|String|ToString(Integer) _damage) true true "(R=1.000000,G=0.099408,B=0.000000,A=1.000000)")
              (bind _dies_ (Default|InflictDamage _gm_battle false _damage (Variables|/Game/GAME/BP/InBattle/Ennemy/BP_BasicWildEnnemy.BP_BasicWildEnnemy_C|GetBPC_CharacterBattleComponent _asbp_basic_wild_ennemy) (Variables|/Game/GAME/BP/InBattle/Manieur_Armes/BP_PlayableCharacterInBattle.BP_PlayableCharacterInBattle_C|GetBPC_PlayableCharacter _asbp_playable_character_in_battle) _is_effective_ false))
              (if _dies_
                (Default|Dies (Variables|/Game/GAME/BP/Components_Interfaces/BPC_PlayableCharacter.BPC_PlayableCharacter_C|GetAlly%20Arme%20/%20Manieur (Variables|/Game/GAME/BP/InBattle/Manieur_Armes/BP_PlayableCharacterInBattle.BP_PlayableCharacterInBattle_C|GetBPC_PlayableCharacter _asbp_playable_character_in_battle))))
              (bind (_damage_2 _is_effective__2) (Default|CalcDamage _asbp_basic_wild_ennemy (Variables|/Game/GAME/BP/Components_Interfaces/BPC_PlayableCharacter.BPC_PlayableCharacter_C|GetAlly%20Arme%20/%20Manieur (Variables|/Game/GAME/BP/InBattle/Manieur_Armes/BP_PlayableCharacterInBattle.BP_PlayableCharacterInBattle_C|GetBPC_PlayableCharacter _asbp_playable_character_in_battle)) _move false))
              (Development|PrintString (Utilities|String|ToString(Integer) _damage_2) true true "(R=1.000000,G=0.099408,B=0.000000,A=1.000000)")
              (bind _dies__2 (Default|InflictDamage _gm_battle false _damage_2 (Variables|/Game/GAME/BP/InBattle/Ennemy/BP_BasicWildEnnemy.BP_BasicWildEnnemy_C|GetBPC_CharacterBattleComponent _asbp_basic_wild_ennemy) (Variables|/Game/GAME/BP/InBattle/Manieur_Armes/BP_PlayableCharacterInBattle.BP_PlayableCharacterInBattle_C|GetBPC_PlayableCharacter (Variables|/Game/GAME/BP/Components_Interfaces/BPC_PlayableCharacter.BPC_PlayableCharacter_C|GetAlly%20Arme%20/%20Manieur (Variables|/Game/GAME/BP/InBattle/Manieur_Armes/BP_PlayableCharacterInBattle.BP_PlayableCharacterInBattle_C|GetBPC_PlayableCharacter _asbp_playable_character_in_battle))) _is_effective__2 false))
              (if _dies__2
                (Default|Dies _asbp_playable_character_in_battle))
              (bind _asbp_basic_wild_ennemy_2 (Utilities|Casting|CastToBP_BasicWildEnnemy (Components|GetOwner (Variables|Default|GetBPC_Attacker))))
              (Default|EndMyTurn _asbp_basic_wild_ennemy_2)
              (else
                (bind (_damage_3 _is_effective__3) (Default|CalcDamage _asbp_basic_wild_ennemy (select (Variables|/Game/GAME/BP/InBattle/BP_InBattlePawn.BP_InBattlePawn_C|GetIsGuardUp? _bp_inbattlepawn) (Variables|/Game/GAME/BP/Components_Interfaces/BPC_PlayableCharacter.BPC_PlayableCharacter_C|GetAlly%20Arme%20/%20Manieur (Variables|/Game/GAME/BP/InBattle/Manieur_Armes/BP_PlayableCharacterInBattle.BP_PlayableCharacterInBattle_C|GetBPC_PlayableCharacter _asbp_playable_character_in_battle)) _asbp_playable_character_in_battle) _move false))
                (Development|PrintString (Utilities|String|Append (Utilities|GetDisplayName (Components|GetOwner (Variables|/Game/GAME/BP/InBattle/Manieur_Armes/BP_PlayableCharacterInBattle.BP_PlayableCharacterInBattle_C|GetBPC_PlayableCharacter (select (Variables|/Game/GAME/BP/InBattle/BP_InBattlePawn.BP_InBattlePawn_C|GetIsGuardUp? _bp_inbattlepawn) (Variables|/Game/GAME/BP/Components_Interfaces/BPC_PlayableCharacter.BPC_PlayableCharacter_C|GetAlly%20Arme%20/%20Manieur (Variables|/Game/GAME/BP/InBattle/Manieur_Armes/BP_PlayableCharacterInBattle.BP_PlayableCharacterInBattle_C|GetBPC_PlayableCharacter _asbp_playable_character_in_battle)) _asbp_playable_character_in_battle)))) " : " (Utilities|String|ToString(Integer) _damage_3)) true true "(R=1.000000,G=0.099408,B=0.000000,A=1.000000)")
                (bind _dies__3 (Default|InflictDamage _gm_battle false _damage_3 (Variables|/Game/GAME/BP/InBattle/Ennemy/BP_BasicWildEnnemy.BP_BasicWildEnnemy_C|GetBPC_CharacterBattleComponent _asbp_basic_wild_ennemy) (Variables|/Game/GAME/BP/InBattle/Manieur_Armes/BP_PlayableCharacterInBattle.BP_PlayableCharacterInBattle_C|GetBPC_PlayableCharacter (select (Variables|/Game/GAME/BP/InBattle/BP_InBattlePawn.BP_InBattlePawn_C|GetIsGuardUp? _bp_inbattlepawn) (Variables|/Game/GAME/BP/Components_Interfaces/BPC_PlayableCharacter.BPC_PlayableCharacter_C|GetAlly%20Arme%20/%20Manieur (Variables|/Game/GAME/BP/InBattle/Manieur_Armes/BP_PlayableCharacterInBattle.BP_PlayableCharacterInBattle_C|GetBPC_PlayableCharacter _asbp_playable_character_in_battle)) _asbp_playable_character_in_battle)) _is_effective__3 false))
                (if _dies__3
                  (Default|Dies (select (Variables|/Game/GAME/BP/InBattle/BP_InBattlePawn.BP_InBattlePawn_C|GetIsGuardUp? _bp_inbattlepawn) (Variables|/Game/GAME/BP/Components_Interfaces/BPC_PlayableCharacter.BPC_PlayableCharacter_C|GetAlly%20Arme%20/%20Manieur (Variables|/Game/GAME/BP/InBattle/Manieur_Armes/BP_PlayableCharacterInBattle.BP_PlayableCharacterInBattle_C|GetBPC_PlayableCharacter _asbp_playable_character_in_battle)) _asbp_playable_character_in_battle))
                  (goto _label)
                  (else
                    (goto _label)))))))))
    (:CastFailed
      (bind _asbp_playable_character_in_battle_2 (Utilities|Casting|CastToBP_PlayableCharacterInBattle (Components|GetOwner (Variables|Default|GetBPC_Attacker))))
      (bind _asbp_basic_wild_ennemy_3 (Utilities|Casting|CastToBP_BasicWildEnnemy (Components|GetOwner _bpc_target)))
      (bind (_damages _effective_) (Default|CalculateAttackDamage _gm_battle (.type _move_infos) (Default|GetStat+Buff _gm_battle "NewEnumerator1" (Variables|/Game/GAME/BP/InBattle/Ennemy/BP_BasicWildEnnemy.BP_BasicWildEnnemy_C|GetBPC_CharacterBattleComponent _asbp_basic_wild_ennemy_3) (Variables|/Game/GAME/BP/InBattle/Manieur_Armes/BP_PlayableCharacterInBattle.BP_PlayableCharacterInBattle_C|GetBPC_PlayableCharacter _asbp_playable_character_in_battle_2) false) (Default|GetStat+Buff _gm_battle "NewEnumerator3" (Variables|/Game/GAME/BP/InBattle/Ennemy/BP_BasicWildEnnemy.BP_BasicWildEnnemy_C|GetBPC_CharacterBattleComponent _asbp_basic_wild_ennemy_3) (Variables|/Game/GAME/BP/InBattle/Manieur_Armes/BP_PlayableCharacterInBattle.BP_PlayableCharacterInBattle_C|GetBPC_PlayableCharacter _asbp_playable_character_in_battle_2) true) (.power _move_infos) 1 (Variables|/Game/GAME/BP/Components_Interfaces/BPC_PlayableCharacter.BPC_PlayableCharacter_C|GetLevel (Variables|/Game/GAME/BP/InBattle/Manieur_Armes/BP_PlayableCharacterInBattle.BP_PlayableCharacterInBattle_C|GetBPC_PlayableCharacter _asbp_playable_character_in_battle_2)) (Variables|/Game/GAME/BP/Components_Interfaces/BPC_WildEnnemy.BPC_WildEnnemy_C|GetElement (Variables|/Game/GAME/BP/InBattle/Ennemy/BP_BasicWildEnnemy.BP_BasicWildEnnemy_C|GetBPC_CharacterBattleComponent _asbp_basic_wild_ennemy_3)) (.element _move_infos)))
      (bind _dies__4 (Default|InflictDamage _gm_battle true _damages (Variables|/Game/GAME/BP/InBattle/Ennemy/BP_BasicWildEnnemy.BP_BasicWildEnnemy_C|GetBPC_CharacterBattleComponent _asbp_basic_wild_ennemy_3) (Variables|/Game/GAME/BP/InBattle/Manieur_Armes/BP_PlayableCharacterInBattle.BP_PlayableCharacterInBattle_C|GetBPC_PlayableCharacter _asbp_playable_character_in_battle_2) _effective_ false))
      (if _dies__4
        (bind _victory_ (Default|KillEnnemy _gm_battle (Variables|/Game/GAME/BP/InBattle/Ennemy/BP_BasicWildEnnemy.BP_BasicWildEnnemy_C|GetBPC_CharacterBattleComponent _asbp_basic_wild_ennemy_3)))
        (if _victory_
          (Utilities|IsValid _bp_inbattlepawn_2
            (:Is%20Valid
              (Default|Victory _bp_inbattlepawn_2))
            (:Is%20Not%20Valid
              (Development|PrintString "pas valide")))
          (else
            (if (== (.nb_oftarget _move_infos) 99) :!label _label_2
              (Default|EndMyTurn _bp_inbattlepawn_2 :!label _label_3)
              (Utilities|FlowControl|Delay 1.0)
              (Transformation|SetRelativeRotation (Variables|/Game/GAME/BP/InBattle/Manieur_Armes/BP_PlayableCharacterInBattle.BP_PlayableCharacterInBattle_C|GetSkeletalMesh _asbp_playable_character_in_battle_2) "0, 0, 0" false false)
              (Transformation|SetRelativeRotation (Variables|/Game/GAME/BP/InBattle/Ennemy/BP_BasicWildEnnemy.BP_BasicWildEnnemy_C|GetSkeletalMesh _asbp_basic_wild_ennemy_3) "0, 0, 0" false false)
              (elif (< (Variables|/Game/GAME/BP/InBattle/BP_InBattlePawn.BP_InBattlePawn_C|GetTemp_NumberOfTargetChoosed _bp_inbattlepawn_2) 0)
                (Variables|/Game/GAME/BP/InBattle/BP_InBattlePawn.BP_InBattlePawn_C|SetCanCancelAttack? _bp_inbattlepawn_2 false)
                (else
                  (goto _label_3))))))
        (else
          (goto _label_2))))))

(event EventBeginPlay
  (EventDispatchers|BindEventtoHitEnnemy (delegate Custom|HitEnnemy_Event)))

(event EventTick
  (params (DeltaSeconds :type Float%20%28single-precision%29)))