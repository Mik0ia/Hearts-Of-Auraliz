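; Random encounter zone that starts battles as the overworld player walks inside its box.
; While the player overlaps it, a throttled Tick samples position every 0.1 seconds and counts sufficient movement as a step.
; At a threshold from GetRandomStepsForBattle, it resets the count, disables input and has the player launch a random battle row.
; Battle table, row choices and average step count come from MasterEncounter at BeginPlay.
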(event OnComponentBeginOverlap(Box)
  (params (OverlappedComponent :type Primitive%20Component%20Object%20Reference) (OtherActor :type Actor%20Object%20Reference) (OtherComp :type Primitive%20Component%20Object%20Reference) (OtherBodyIndex :type Integer) (bFromSweep :type Boolean) (SweepResult :type Hit%20Result%20Structure%20%28by%20ref%29))
  (Utilities|IsValid (Actor|GetComponentbyClass OtherActor "/Game/GAME/BP/Components_Interfaces/BPC_PlayerOverworld.BPC_PlayerOverworld_C")
    (:Is%20Valid
      (Variables|Default|SetPlayerIsInside true)
      (bind _asbp_player_character (Utilities|Casting|CastToBP_PlayerCharacter OtherActor))
      (bind _output_get (Variables|Default|SetAs%20BP%20Player%20Character _asbp_player_character))
      (Variables|Default|SetPlayerOldLocation (Transformation|GetActorLocation _output_get)))))

(event OnComponentEndOverlap(Box)
  (params (OverlappedComponent :type Primitive%20Component%20Object%20Reference) (OtherActor :type Actor%20Object%20Reference) (OtherComp :type Primitive%20Component%20Object%20Reference) (OtherBodyIndex :type Integer))
  (Utilities|IsValid (Actor|GetComponentbyClass OtherActor "/Game/GAME/BP/Components_Interfaces/BPC_PlayerOverworld.BPC_PlayerOverworld_C")
    (:Is%20Valid
      (Variables|Default|SetPlayerIsInside false))))

(event Custom|WalkEvent
  (bind _output_get (Variables|Default|SetCurrentStepCount (+ (Variables|Default|GetCurrentStepCount) 1)))
  (if (>= _output_get (Variables|Default|GetNextBattleNumberOfSteps))
    (CallFunction|LaunchBattle)))

(event Custom|LaunchBattle
  (bind _indexofrandombattle (Variables|Default|GetIndexOfRandomBattle))
  (Input|DisableInput (Variables|Default|GetAs%20BP%20Player%20Character) 0)
  (Variables|Default|SetCurrentStepCount 0)
  (Variables|Default|SetNextBattleNumberOfSteps (Utilities|GetRandomStepsforBattle (Variables|Default|GetAverageStepBattleCount)))
  (Default|LaunchBattle (Variables|Default|GetAs%20BP%20Player%20Character) (Utilities|Array|Get(acopy) _indexofrandombattle (Math|Random|RandomIntegerinRange 0 (- (Utilities|Array|Length _indexofrandombattle) 1))) (Variables|Default|GetBattleTable)))

(event EventTick
  (params (DeltaSeconds :type Float%20%28single-precision%29))
  (bind _as_bp_player_character (Variables|Default|GetAs%20BP%20Player%20Character))
  (bind _returnvalue (Transformation|GetActorLocation _as_bp_player_character))
  (if (Variables|Default|GetPlayerIsInside)
    (Utilities|FlowControl|DoOnce false :!label _label
      (:Completed
        (if (>= (Math|Float|Absolute(Float) (Math|Vector|VectorLength (- _returnvalue (Variables|Default|GetPlayerOldLocation)))) 1e+01)
          (CallFunction|WalkEvent))
        (Variables|Default|SetPlayerOldLocation _returnvalue)
        (Utilities|FlowControl|Delay 0.1)
        (goto _label Reset)))))

(event EventBeginPlay
  (bind _masterencounter (Variables|Default|GetMasterEncounter))
  (bind _output_get (Variables|Default|SetAverageStepBattleCount (Variables|/Game/GAME/BP/Encounter/BP_MasterRandomEncounter.BP_MasterRandomEncounter_C|GetStepValueAverage _masterencounter)))
  (Variables|Default|SetBattleTable (Variables|/Game/GAME/BP/Encounter/BP_MasterRandomEncounter.BP_MasterRandomEncounter_C|GetRandomBattleTable _masterencounter))
  (Variables|Default|SetIndexOfRandomBattle (Variables|/Game/GAME/BP/Encounter/BP_MasterRandomEncounter.BP_MasterRandomEncounter_C|GetRowBattleIndex _masterencounter))
  (Variables|Default|SetNextBattleNumberOfSteps (Utilities|GetRandomStepsforBattle _output_get)))

(fn ConstructionScript)