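; Battle game mode that sets up an RPG fight from the GameInstance's battle row, including enemies, levels and music.
; On BeginPlay it spawns the player's Manieur/Arme (wielder/weapon) duos, linked as allies, and the enemies at team-size-based RootManager roots.
; Data tables supply classes, level-scaled stats, level-gated moves and talents, which are attached as runtime components.
; Helpers return battlers by index and print debug info; move use only prints so far.
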(event EventBeginPlay
  (bind _outactors (Actor|GetAllActorsOfClass "/Game/GAME/BP/InBattle/BP_RootManager.BP_RootManager_C"))
  (Variables|Default|SetRootManager (Utilities|Array|Get(acopy) _outactors))
  (CallFunction|GetBattleInfo)
  (Audio|PlaySound2D (Variables|Default|GetBattle%20Music) 1.0 1.0 0.0 0 0)
  (CallFunction|SpawnPlayerTeam)
  (CallFunction|SpawnEnnemyTeam))

(event EventTick
  (params (DeltaSeconds :type Float%20%28single-precision%29)))

(fn ConstructionScript
  (bind _asgi_game_instance (Utilities|Casting|CastToGI_GameInstance (Game|GetGameInstance)))
  (Variables|Default|SetGI%20Game%20Instance%20REF _asgi_game_instance))

(fn GetBattleInfo
  (bind _gi_game_instance_ref (Variables|Default|GetGI%20Game%20Instance%20REF))
  (bind _current_battle_row___ref (Variables|/Game/GAME/BP/General/GI_GameInstance.GI_GameInstance_C|GetCurrent%20Battle%20Row%20+%20Ref _gi_game_instance_ref))
  (Utilities|Array|Clear (Variables|Default|GetEnnemy%20Refs))
  (Utilities|Array|Clear (Variables|Default|GetEnnemys%20Levels))
  (bind _values (Utilities|Map|Values _current_battle_row___ref))
  (bind _keys (Utilities|Map|Keys _current_battle_row___ref))
  (bind _returnvalue (Utilities|GetDataTableRow (Utilities|Array|Get(acopy) _values) (Utilities|String|StringToName (Utilities|String|ToString(Integer) (Utilities|Array|Get(acopy) _keys))))
    (:then
      (Variables|Default|SetEnnemy%20Refs (.EnnemyRefs (Utilities|Struct|BreakST_WildBattle _returnvalue)))
      (Variables|Default|SetEnnemys%20Levels (.EnnemysLevels (Utilities|Struct|BreakST_WildBattle _returnvalue)))
      (Variables|Default|SetBattle%20Music (.BattleMusic (Utilities|Struct|BreakST_WildBattle _returnvalue)))
      (Variables|Default|SetBattle%20Text (.BattleText (Utilities|Struct|BreakST_WildBattle _returnvalue)))
      (Variables|Default|SetCan%20Escape? (.CanEscape? (Utilities|Struct|BreakST_WildBattle _returnvalue))))))

(fn SpawnPlayerTeam
  (Utilities|Array|Clear (Variables|Default|GetPlayableCharacterBP_Refs))
  (bind _outrownames (DataTable|GetDataTableRowNames "/Game/GAME/DATA/DATA_TABLE/DT_PlayerTeam.DT_PlayerTeam"))
  (bind _roots_refs (CallFunction|GetPlayersRoots (Utilities|Array|Length _outrownames)))
  (LocalVariables|SetRootRefs _roots_refs)
  (for (_array_element _array_index) _outrownames
    (bind _returnvalue (Utilities|GetDataTableRow "/Game/GAME/DATA/DATA_TABLE/DT_PlayerTeam.DT_PlayerTeam" _array_element)
      (:then
        (bind _outrownames_2 (DataTable|GetDataTableRowNames "/Game/GAME/DATA/DATA_TABLE/DT_DuoTable.DT_DuoTable"))
        (bind _array_element_2 (Utilities|Array|ForEachLoopwithBreak _outrownames_2 :!label _label)
          (:LoopBody
            (bind _returnvalue_2 (Utilities|GetDataTableRow "/Game/GAME/DATA/DATA_TABLE/DT_DuoTable.DT_DuoTable" _array_element_2)
              (:then
                (if (Utilities|Enum|Equal(Enum) (.DuoEnum (Utilities|Struct|BreakST_DuoCharacter _returnvalue_2)) (.DuoRef (Utilities|Struct|BreakST_PlayerTeam _returnvalue)))
                  (if (Utilities|Enum|NotEqual(Enum) (.Manieur (Utilities|Struct|BreakST_DuoCharacter _returnvalue_2)) "NewEnumerator5")
                    (LocalVariables|SetManieur (.Manieur (Utilities|Struct|BreakST_DuoCharacter _returnvalue_2)))
                    (else
                      (LocalVariables|SetManieur "NewEnumerator5")))
                  (if (Utilities|Enum|NotEqual(Enum) (.Arme (Utilities|Struct|BreakST_DuoCharacter _returnvalue_2)) "NewEnumerator5")
                    (LocalVariables|SetArme (.Arme (Utilities|Struct|BreakST_DuoCharacter _returnvalue_2)))
                    (goto _label Break)
                    (else
                      (LocalVariables|SetArme "NewEnumerator5")
                      (goto _label Break)))))))
          (:Completed
            (Development|PrintString (Utilities|String|Append "Manieur : " (Utilities|String|EnumtoString (LocalVariables|GetManieur))))
            (Development|PrintString (Utilities|String|Append "Arme : " (Utilities|String|EnumtoString (LocalVariables|GetArme))))
            (if (Utilities|Enum|NotEqual(Enum) (LocalVariables|GetManieur) "NewEnumerator5")
              (bind _returnvalue_3 (Utilities|GetDataTableRow "/Game/GAME/DATA/DATA_TABLE/DT_BattleRefs.DT_BattleRefs" (Utilities|String|StringToName (Utilities|String|EnumtoString (LocalVariables|GetManieur))))
                (:then
                  (bind _returnvalue_4 (Game|SpawnActorfromClass (.BP_Ref (Utilities|Struct|BreakST_InBattleRefs _returnvalue_3)) (Math|Transform|MakeTransform (.location (Transformation|GetActorTransform (Utilities|Array|Get(acopy) (LocalVariables|GetRootRefs) _array_index))) (.rotation (Transformation|GetActorTransform (Utilities|Array|Get(acopy) (LocalVariables|GetRootRefs) _array_index))) (.Scale (Utilities|Struct|BreakST_InBattleRefs _returnvalue_3))) "AlwaysSpawn" "MultiplyWithRoot" 0 0))
                  (bind _asbp_playable_character_in_battle (Utilities|Casting|CastToBP_PlayableCharacterInBattle _returnvalue_4))
                  (Utilities|Array|Add (Variables|Default|GetPlayableCharacterBP_Refs) _asbp_playable_character_in_battle)
                  (bind _returnvalue_5 (Utilities|GetDataTableRow "/Game/GAME/DATA/DATA_TABLE/DT_PlayerTeam.DT_PlayerTeam" (Utilities|String|StringToName (Utilities|String|EnumtoString (LocalVariables|GetManieur))))
                    (:then
                      (CallFunction|SetPlayableCharacterInfo _asbp_playable_character_in_battle (Utilities|String|StringToName (Utilities|String|EnumtoString (LocalVariables|GetManieur))) (.Level (Utilities|Struct|BreakST_PlayerTeam _returnvalue_5)) (.ManieurLostHp (Utilities|Struct|BreakST_PlayerTeam _returnvalue_5)) (.ArmeLostHP (Utilities|Struct|BreakST_PlayerTeam _returnvalue_5)) true)
                      (if (Utilities|Enum|NotEqual(Enum) (LocalVariables|GetArme) "NewEnumerator5")
                        (bind _returnvalue_6 (Utilities|GetDataTableRow "/Game/GAME/DATA/DATA_TABLE/DT_BattleRefs.DT_BattleRefs" (Utilities|String|StringToName (Utilities|String|EnumtoString (LocalVariables|GetArme))))
                          (:then
                            (bind _returnvalue_7 (Game|SpawnActorfromClass (.BP_Ref (Utilities|Struct|BreakST_InBattleRefs _returnvalue_6)) (Math|Transform|MakeTransform (.location (Transformation|GetWorldTransform (Variables|/Game/GAME/BP/InBattle/Manieur_Armes/BP_PlayableCharacterInBattle.BP_PlayableCharacterInBattle_C|GetArme_Root _asbp_playable_character_in_battle))) (.rotation (Transformation|GetWorldTransform (Variables|/Game/GAME/BP/InBattle/Manieur_Armes/BP_PlayableCharacterInBattle.BP_PlayableCharacterInBattle_C|GetArme_Root _asbp_playable_character_in_battle))) (.Scale (Utilities|Struct|BreakST_InBattleRefs _returnvalue_6))) "AlwaysSpawn" "MultiplyWithRoot" 0 0))
                            (bind _asbp_playable_character_in_battle_2 (Utilities|Casting|CastToBP_PlayableCharacterInBattle _returnvalue_7))
                            (Utilities|Array|Add (Variables|Default|GetPlayableCharacterBP_Refs) _asbp_playable_character_in_battle_2)
                            (bind _returnvalue_8 (Utilities|GetDataTableRow "/Game/GAME/DATA/DATA_TABLE/DT_PlayerTeam.DT_PlayerTeam" (Utilities|String|StringToName (Utilities|String|EnumtoString (LocalVariables|GetManieur))))
                              (:then
                                (CallFunction|SetPlayableCharacterInfo _asbp_playable_character_in_battle_2 (Utilities|String|StringToName (Utilities|String|EnumtoString (LocalVariables|GetArme))) (.Level (Utilities|Struct|BreakST_PlayerTeam _returnvalue_8)) (.ManieurLostHp (Utilities|Struct|BreakST_PlayerTeam _returnvalue_8)) (.ArmeLostHP (Utilities|Struct|BreakST_PlayerTeam _returnvalue_8)) false)
                                (Variables|/Game/GAME/BP/Components_Interfaces/BPC_PlayableCharacter.BPC_PlayableCharacter_C|SetAlly%20Arme%20/%20Manieur (Variables|/Game/GAME/BP/InBattle/Manieur_Armes/BP_PlayableCharacterInBattle.BP_PlayableCharacterInBattle_C|GetBPC_PlayableCharacter _asbp_playable_character_in_battle) _asbp_playable_character_in_battle_2)
                                (Variables|/Game/GAME/BP/Components_Interfaces/BPC_PlayableCharacter.BPC_PlayableCharacter_C|SetAlly%20Arme%20/%20Manieur (Variables|/Game/GAME/BP/InBattle/Manieur_Armes/BP_PlayableCharacterInBattle.BP_PlayableCharacterInBattle_C|GetBPC_PlayableCharacter _asbp_playable_character_in_battle_2) _asbp_playable_character_in_battle)))))))))))))))))

(fn GetPlayersRoots
  (params (Size%20of%20the%20Team :type Integer))
  (bind _rootmanager (Variables|Default|GetRootManager))
  (switch int Size%20of%20the%20Team
    (:1
      (return (Variables|/Game/GAME/BP/InBattle/BP_RootManager.BP_RootManager_C|Get1PCharacterRoot _rootmanager)))
    (:2
      (return (Variables|/Game/GAME/BP/InBattle/BP_RootManager.BP_RootManager_C|Get2PCharacterRoot _rootmanager)))
    (:3
      (return (Variables|/Game/GAME/BP/InBattle/BP_RootManager.BP_RootManager_C|Get3PCharacterRoot _rootmanager)))))

(fn SetPlayableCharacterInfo
  (params (Character%20Ref :type BP%20Playable%20Character%20in%20Battle%20Object%20Reference) (RowName :type Name) (LV :type Integer) (M_LostHP :type Integer) (A_LostHP :type Integer) (Manieur? :type Boolean))
  (bind _bpc_playablecharacter (Variables|/Game/GAME/BP/InBattle/Manieur_Armes/BP_PlayableCharacterInBattle.BP_PlayableCharacterInBattle_C|GetBPC_PlayableCharacter Character%20Ref))
  (bind _returnvalue (Utilities|GetDataTableRow "/Game/GAME/DATA/DATA_TABLE/DT_PlayableCharacterBaseStats.DT_PlayableCharacterBaseStats" RowName)
    (:then
      ;[0.15 0.15 0.15 0.5] statistiques
      (bind _current_stat (CallFunction|SetHPstat (.Base_PV (Utilities|Struct|BreakST_PlayableCharacter _returnvalue)) LV))
      (Variables|/Game/GAME/BP/Components_Interfaces/BPC_PlayableCharacter.BPC_PlayableCharacter_C|SetIsManieur? _bpc_playablecharacter Manieur?)
      (bind _output_get (Variables|/Game/GAME/BP/Components_Interfaces/BPC_PlayableCharacter.BPC_PlayableCharacter_C|SetBase%20HP _bpc_playablecharacter _current_stat))
      (if Manieur?
        (Variables|/Game/GAME/BP/Components_Interfaces/BPC_PlayableCharacter.BPC_PlayableCharacter_C|Setcurrent%20HP _bpc_playablecharacter (- _output_get M_LostHP))
        (else
          (Variables|/Game/GAME/BP/Components_Interfaces/BPC_PlayableCharacter.BPC_PlayableCharacter_C|Setcurrent%20HP _bpc_playablecharacter (- _output_get A_LostHP))))
      (Variables|/Game/GAME/BP/Components_Interfaces/BPC_PlayableCharacter.BPC_PlayableCharacter_C|SetLevel _bpc_playablecharacter LV)
      (bind _current_stat_2 (CallFunction|SetStat (.Base_FOR (Utilities|Struct|BreakST_PlayableCharacter _returnvalue)) LV))
      (Variables|/Game/GAME/BP/Components_Interfaces/BPC_PlayableCharacter.BPC_PlayableCharacter_C|SetBase%20FOR _bpc_playablecharacter _current_stat_2)
      (bind _current_stat_3 (CallFunction|SetStat (.Base_DEF (Utilities|Struct|BreakST_PlayableCharacter _returnvalue)) LV))
      (Variables|/Game/GAME/BP/Components_Interfaces/BPC_PlayableCharacter.BPC_PlayableCharacter_C|SetBase%20DEF _bpc_playablecharacter _current_stat_3)
      (bind _current_stat_4 (CallFunction|SetStat (.Base_MAG (Utilities|Struct|BreakST_PlayableCharacter _returnvalue)) LV))
      (Variables|/Game/GAME/BP/Components_Interfaces/BPC_PlayableCharacter.BPC_PlayableCharacter_C|SetBase%20MAG _bpc_playablecharacter _current_stat_4)
      (bind _current_stat_5 (CallFunction|SetStat (.Base_DEFM (Utilities|Struct|BreakST_PlayableCharacter _returnvalue)) LV))
      (Variables|/Game/GAME/BP/Components_Interfaces/BPC_PlayableCharacter.BPC_PlayableCharacter_C|SetBase%20DEF_M _bpc_playablecharacter _current_stat_5)
      (bind _current_stat_6 (CallFunction|SetStat (.Base_VIT (Utilities|Struct|BreakST_PlayableCharacter _returnvalue)) LV))
      (Variables|/Game/GAME/BP/Components_Interfaces/BPC_PlayableCharacter.BPC_PlayableCharacter_C|SetBase%20VIT _bpc_playablecharacter _current_stat_6)
      (CallFunction|SetUsableMoves (.MovePool (Utilities|Struct|BreakST_PlayableCharacter _returnvalue)) LV 0 _bpc_playablecharacter false)
      (bind _output_get_2 (Variables|/Game/GAME/BP/Components_Interfaces/BPC_PlayableCharacter.BPC_PlayableCharacter_C|SetTalent _bpc_playablecharacter (.Talent (Utilities|Struct|BreakST_PlayableCharacter _returnvalue))))
      (Variables|/Game/GAME/BP/Components_Interfaces/BPC_PlayableCharacter.BPC_PlayableCharacter_C|SetElement _bpc_playablecharacter (.Element (Utilities|Struct|BreakST_PlayableCharacter _returnvalue)))
      (Variables|/Game/GAME/BP/Components_Interfaces/BPC_PlayableCharacter.BPC_PlayableCharacter_C|SetCharacterRef _bpc_playablecharacter (.Character (Utilities|Struct|BreakST_PlayableCharacter _returnvalue)))
      (Variables|/Game/GAME/BP/Components_Interfaces/BPC_PlayableCharacter.BPC_PlayableCharacter_C|SetLevel _bpc_playablecharacter LV)
      (bind _outrownames (DataTable|GetDataTableRowNames "/Game/GAME/DATA/DATA_TABLE/DT_TalentInfo.DT_TalentInfo"))
      (for _array_element _outrownames
        (bind _returnvalue_2 (Utilities|GetDataTableRow "/Game/GAME/DATA/DATA_TABLE/DT_TalentInfo.DT_TalentInfo" _array_element)
          (:then
            (if (Utilities|Enum|Equal(Enum) (.TalentEnum (Utilities|Struct|BreakST_TalentInfo _returnvalue_2)) _output_get_2)
              (Variables|/Game/GAME/BP/Components_Interfaces/BPC_PlayableCharacter.BPC_PlayableCharacter_C|SetTalentActivation (Variables|/Game/GAME/BP/InBattle/Manieur_Armes/BP_PlayableCharacterInBattle.BP_PlayableCharacterInBattle_C|GetBPC_PlayableCharacter Character%20Ref) (.TalentActivations (Utilities|Struct|BreakST_TalentInfo _returnvalue_2)))
              (Game|AddComponentbyClass Character%20Ref (.BPC_Related (Utilities|Struct|BreakST_TalentInfo _returnvalue_2))))))))))

(fn SpawnEnnemyTeam
  (bind _ennemy_refs (Variables|Default|GetEnnemy%20Refs))
  (Utilities|Array|Clear (Variables|Default|GetEnnemyBP_Refs))
  (bind _roots_refs (CallFunction|GetEnnemyRoots (Utilities|Array|Length _ennemy_refs)))
  (LocalVariables|SetRoots%20Refs _roots_refs)
  (for (_array_element _array_index) _ennemy_refs
    (bind _returnvalue (Utilities|GetDataTableRow "/Game/GAME/DATA/DATA_TABLE/DT_WildInBattleRefs.DT_WildInBattleRefs" (Utilities|String|StringToName (Utilities|String|EnumtoString _array_element)))
      (:then
        (bind _returnvalue_2 (Game|SpawnActorfromClass (.BP_Ref (Utilities|Struct|BreakST_WildInBattleRefs _returnvalue)) (Math|Transform|MakeTransform (.location (Transformation|GetActorTransform (Utilities|Array|Get(acopy) (LocalVariables|GetRoots%20Refs) _array_index))) (.rotation (Transformation|GetActorTransform (Utilities|Array|Get(acopy) (LocalVariables|GetRoots%20Refs) _array_index))) (.Scale (Utilities|Struct|BreakST_WildInBattleRefs _returnvalue))) "AlwaysSpawn" "MultiplyWithRoot" 0 0))
        (bind _asbp_basic_wild_ennemy (Utilities|Casting|CastToBP_BasicWildEnnemy _returnvalue_2))
        (Utilities|Array|Add (Variables|Default|GetEnnemyBP_Refs) _asbp_basic_wild_ennemy)
        (CallFunction|SetEnnemyInfo _asbp_basic_wild_ennemy (Utilities|String|StringToName (Utilities|String|EnumtoString _array_element)) (Utilities|Array|Get(acopy) (Variables|Default|GetEnnemys%20Levels) _array_index))))))

(fn SetStat
  (params (Base%20Stat :type Integer) (Level :type Integer))
  (return (+ (/ (* (* Base%20Stat 2) Level) 100) 1)))

(fn GetEnnemyRoots
  (params (Size%20of%20the%20Team :type Integer))
  (bind _rootmanager (Variables|Default|GetRootManager))
  (switch int Size%20of%20the%20Team
    (:1
      (return (Variables|/Game/GAME/BP/InBattle/BP_RootManager.BP_RootManager_C|Get1ECharacterRoot _rootmanager)))
    (:2
      (return (Variables|/Game/GAME/BP/InBattle/BP_RootManager.BP_RootManager_C|Get2ECharacterRoot _rootmanager)))
    (:3
      (return (Variables|/Game/GAME/BP/InBattle/BP_RootManager.BP_RootManager_C|Get3ECharacterRoot _rootmanager)))
    (:4
      (return (Variables|/Game/GAME/BP/InBattle/BP_RootManager.BP_RootManager_C|Get4ECharacterRoot _rootmanager)))
    (:5
      (return (Variables|/Game/GAME/BP/InBattle/BP_RootManager.BP_RootManager_C|Get5ECharacterRoot _rootmanager)))))

(fn SetEnnemyInfo
  (params (Character%20Ref :type BP%20Basic%20Wild%20Ennemy%20Object%20Reference) (RowName :type Name) (LV :type Integer))
  (bind _bpc_characterbattlecomponent (Variables|/Game/GAME/BP/InBattle/Ennemy/BP_BasicWildEnnemy.BP_BasicWildEnnemy_C|GetBPC_CharacterBattleComponent Character%20Ref))
  (bind _returnvalue (Utilities|GetDataTableRow "/Game/GAME/DATA/DATA_TABLE/DT_WildEnnemyTabl.DT_WildEnnemyTabl" RowName)
    (:then
      (Variables|/Game/GAME/BP/Components_Interfaces/BPC_WildEnnemy.BPC_WildEnnemy_C|SetRace _bpc_characterbattlecomponent (.Ennemy (Utilities|Struct|BreakST_WildEnnemy _returnvalue)))
      ;[0.15 0.15 0.15 0.5] statistiques
      (bind _current_stat (CallFunction|SetHPstat (.Base_PV (Utilities|Struct|BreakST_WildEnnemy _returnvalue)) LV))
      (bind _output_get (Variables|/Game/GAME/BP/Components_Interfaces/BPC_WildEnnemy.BPC_WildEnnemy_C|SetBase%20HP _bpc_characterbattlecomponent _current_stat))
      (Variables|/Game/GAME/BP/Components_Interfaces/BPC_WildEnnemy.BPC_WildEnnemy_C|Setcurrent%20HP _bpc_characterbattlecomponent _output_get)
      (Variables|/Game/GAME/BP/Components_Interfaces/BPC_WildEnnemy.BPC_WildEnnemy_C|SetLevel _bpc_characterbattlecomponent LV)
      (bind _current_stat_2 (CallFunction|SetStat (.Base_FOR (Utilities|Struct|BreakST_WildEnnemy _returnvalue)) LV))
      (Variables|/Game/GAME/BP/Components_Interfaces/BPC_WildEnnemy.BPC_WildEnnemy_C|SetBase%20FOR _bpc_characterbattlecomponent _current_stat_2)
      (bind _current_stat_3 (CallFunction|SetStat (.Base_DEF (Utilities|Struct|BreakST_WildEnnemy _returnvalue)) LV))
      (Variables|/Game/GAME/BP/Components_Interfaces/BPC_WildEnnemy.BPC_WildEnnemy_C|SetBase%20DEF _bpc_characterbattlecomponent _current_stat_3)
      (bind _current_stat_4 (CallFunction|SetStat (.Base_MAG (Utilities|Struct|BreakST_WildEnnemy _returnvalue)) LV))
      (Variables|/Game/GAME/BP/Components_Interfaces/BPC_WildEnnemy.BPC_WildEnnemy_C|SetBase%20MAG _bpc_characterbattlecomponent _current_stat_4)
      (bind _current_stat_5 (CallFunction|SetStat (.Base_DEFM (Utilities|Struct|BreakST_WildEnnemy _returnvalue)) LV))
      (Variables|/Game/GAME/BP/Components_Interfaces/BPC_WildEnnemy.BPC_WildEnnemy_C|SetBase%20DEF_M _bpc_characterbattlecomponent _current_stat_5)
      (bind _current_stat_6 (CallFunction|SetStat (.Base_VIT (Utilities|Struct|BreakST_WildEnnemy _returnvalue)) LV))
      (Variables|/Game/GAME/BP/Components_Interfaces/BPC_WildEnnemy.BPC_WildEnnemy_C|SetBase%20VIT _bpc_characterbattlecomponent _current_stat_6)
      (Variables|/Game/GAME/BP/Components_Interfaces/BPC_WildEnnemy.BPC_WildEnnemy_C|SetIQ _bpc_characterbattlecomponent (.IQ (Utilities|Struct|BreakST_WildEnnemy _returnvalue)))
      (CallFunction|SetUsableMoves (.MovePool (Utilities|Struct|BreakST_WildEnnemy _returnvalue)) LV _bpc_characterbattlecomponent 0 true)
      (bind _output_get_2 (Variables|/Game/GAME/BP/Components_Interfaces/BPC_WildEnnemy.BPC_WildEnnemy_C|SetTalent _bpc_characterbattlecomponent (.Talent (Utilities|Struct|BreakST_WildEnnemy _returnvalue))))
      (Variables|/Game/GAME/BP/Components_Interfaces/BPC_WildEnnemy.BPC_WildEnnemy_C|SetElement _bpc_characterbattlecomponent (.Element (Utilities|Struct|BreakST_WildEnnemy _returnvalue)))
      (bind _outrownames (DataTable|GetDataTableRowNames "/Game/GAME/DATA/DATA_TABLE/DT_TalentInfo.DT_TalentInfo"))
      (for _array_element _outrownames
        (bind _returnvalue_2 (Utilities|GetDataTableRow "/Game/GAME/DATA/DATA_TABLE/DT_TalentInfo.DT_TalentInfo" _array_element)
          (:then
            (if (Utilities|Enum|Equal(Enum) (.TalentEnum (Utilities|Struct|BreakST_TalentInfo _returnvalue_2)) _output_get_2)
              (Variables|/Game/GAME/BP/Components_Interfaces/BPC_WildEnnemy.BPC_WildEnnemy_C|SetTalentActivation _bpc_characterbattlecomponent (.TalentActivations (Utilities|Struct|BreakST_TalentInfo _returnvalue_2)))
              (Game|AddComponentbyClass (Components|GetOwner _bpc_characterbattlecomponent) (.BPC_Related (Utilities|Struct|BreakST_TalentInfo _returnvalue_2))))))))))

(fn ReturnBattlerBPC
  (params (Ennemy%20? :type Boolean) (Index :type Integer))
  (bind _ennemybp_refs (Variables|Default|GetEnnemyBP_Refs))
  (bind _playablecharacterbp_refs (Variables|Default|GetPlayableCharacterBP_Refs))
  (if Ennemy%20?
    (if (<= Index (- (Utilities|Array|Length _ennemybp_refs) 1))
      (return (Variables|/Game/GAME/BP/InBattle/Ennemy/BP_BasicWildEnnemy.BP_BasicWildEnnemy_C|GetBPC_CharacterBattleComponent (Utilities|Array|Get(acopy) _ennemybp_refs Index)) 0)
      (else
        (Development|PrintString "Out Of Index")))
    (elif (<= Index (- (Utilities|Array|Length _playablecharacterbp_refs) 1))
      (for _array_element _playablecharacterbp_refs
        (Development|PrintString (Utilities|GetDisplayName _array_element) true true "(R=1.000000,G=0.019892,B=0.000000,A=1.000000)"))
      (return 0 (Variables|/Game/GAME/BP/InBattle/Manieur_Armes/BP_PlayableCharacterInBattle.BP_PlayableCharacterInBattle_C|GetBPC_PlayableCharacter (Utilities|Array|Get(acopy) _playablecharacterbp_refs Index)))
      (else
        (Development|PrintString "Out Of Index")))))

(fn PrintALLINFOBpcEnnemy
  (params (BPC :type BPC%20Wild%20Ennemy%20Object%20Reference))
  (Utilities|StringAppend+Print "Race : " (Utilities|String|EnumtoString (Variables|/Game/GAME/BP/Components_Interfaces/BPC_WildEnnemy.BPC_WildEnnemy_C|GetRace BPC))
    (:Execute%20out
      (Utilities|StringAppend+Print "Élement : " (Utilities|String|EnumtoString (Variables|/Game/GAME/BP/Components_Interfaces/BPC_WildEnnemy.BPC_WildEnnemy_C|GetElement BPC))
        (:Execute%20out
          (Utilities|StringAppend+Print "Talent : " (Utilities|String|EnumtoString (Variables|/Game/GAME/BP/Components_Interfaces/BPC_WildEnnemy.BPC_WildEnnemy_C|GetTalent BPC))
            (:Execute%20out
              (Utilities|StringAppend+Print "HP : " (Utilities|String|Append (Utilities|String|Append (Utilities|String|ToString(Integer) (Variables|/Game/GAME/BP/Components_Interfaces/BPC_WildEnnemy.BPC_WildEnnemy_C|Getcurrent%20HP BPC)) " / ") (Utilities|String|ToString(Integer) (Variables|/Game/GAME/BP/Components_Interfaces/BPC_WildEnnemy.BPC_WildEnnemy_C|GetBase%20HP BPC)))
                (:Execute%20out
                  (Utilities|StringAppend+Print "Level :" (Utilities|String|ToString(Integer) (Variables|/Game/GAME/BP/Components_Interfaces/BPC_WildEnnemy.BPC_WildEnnemy_C|GetLevel BPC))
                    (:Execute%20out
                      (Utilities|StringAppend+Print "FOR :" (Utilities|String|ToString(Integer) (Variables|/Game/GAME/BP/Components_Interfaces/BPC_WildEnnemy.BPC_WildEnnemy_C|GetBase%20FOR BPC))
                        (:Execute%20out
                          (Utilities|StringAppend+Print "DEF :" (Utilities|String|ToString(Integer) (Variables|/Game/GAME/BP/Components_Interfaces/BPC_WildEnnemy.BPC_WildEnnemy_C|GetBase%20DEF BPC))
                            (:Execute%20out
                              (Utilities|StringAppend+Print "MAG : " (Utilities|String|ToString(Integer) (Variables|/Game/GAME/BP/Components_Interfaces/BPC_WildEnnemy.BPC_WildEnnemy_C|GetBase%20MAG BPC))
                                (:Execute%20out
                                  (Utilities|StringAppend+Print "DEF.M :" (Utilities|String|ToString(Integer) (Variables|/Game/GAME/BP/Components_Interfaces/BPC_WildEnnemy.BPC_WildEnnemy_C|GetBase%20DEF_M BPC))
                                    (:Execute%20out
                                      (Utilities|StringAppend+Print "VIT :" (Utilities|String|ToString(Integer) (Variables|/Game/GAME/BP/Components_Interfaces/BPC_WildEnnemy.BPC_WildEnnemy_C|GetBase%20VIT BPC))
                                        (:Execute%20out
                                          (Utilities|StringAppend+Print "IQ :" (Utilities|String|ToString(Integer) (Variables|/Game/GAME/BP/Components_Interfaces/BPC_WildEnnemy.BPC_WildEnnemy_C|GetIQ BPC))
                                            (:Execute%20out
                                              (for (_array_element _array_index) (Variables|/Game/GAME/BP/Components_Interfaces/BPC_WildEnnemy.BPC_WildEnnemy_C|GetUsable%20Moves BPC)
                                                (Utilities|StringAppend+Print (Utilities|String|Append (Utilities|String|Append "Move " (Utilities|String|ToString(Integer) (+ _array_index 1))) " : ") (Utilities|String|EnumtoString _array_element))))))))))))))))))))))))))

(fn SetUsableMoves
  (params (MovePool :type Map%20of%20E_Moves%20Enums%20to%20Integers :default "NewEnumerator0") (LV :type Integer) (BPC_Ref_Ennemy :type BPC%20Wild%20Ennemy%20Object%20Reference) (BPC_Ref_Player :type BPC%20Playable%20Character%20Object%20Reference) (Ennemy? :type Boolean))
  (if Ennemy?
    ;[0.15 0.15 0.15 0.5] if its an ennemy character
    (for _index (range 0 (- (Utilities|Map|Length MovePool) 1))
      (bind _values (Utilities|Map|Values MovePool))
      (if (>= LV (Utilities|Array|Get(acopy) _values _index))
        (bind _keys (Utilities|Map|Keys MovePool))
        (Utilities|Array|Add (Variables|/Game/GAME/BP/Components_Interfaces/BPC_WildEnnemy.BPC_WildEnnemy_C|GetUsable%20Moves BPC_Ref_Ennemy) (Utilities|Array|Get(acopy) _keys _index))))
    (else
      ;[0.15 0.15 0.15 0.5] if its an playable character
      (for _index_2 (range 0 (- (Utilities|Map|Length MovePool) 1))
        (bind _values_2 (Utilities|Map|Values MovePool))
        (if (>= LV (Utilities|Array|Get(acopy) _values_2 _index_2))
          (bind _keys_2 (Utilities|Map|Keys MovePool))
          (Utilities|Array|Add (Variables|/Game/GAME/BP/Components_Interfaces/BPC_PlayableCharacter.BPC_PlayableCharacter_C|GetUsable%20Moves BPC_Ref_Player) (Utilities|Array|Get(acopy) _keys_2 _index_2)))))))

(fn SetHPstat
  (params (Base%20Stat :type Integer) (Level :type Integer))
  (return (+ (+ (/ (* (* Base%20Stat 2) Level) 100) Level) 10)))

(fn PrintALLINFOBpcPlayable
  (params (BPC :type BPC%20Playable%20Character%20Object%20Reference))
  (Utilities|StringAppend+Print "Character : " (Utilities|String|EnumtoString (Variables|/Game/GAME/BP/Components_Interfaces/BPC_PlayableCharacter.BPC_PlayableCharacter_C|GetCharacterRef BPC))
    (:Execute%20out
      (Utilities|StringAppend+Print "Élement : " (Utilities|String|EnumtoString (Variables|/Game/GAME/BP/Components_Interfaces/BPC_PlayableCharacter.BPC_PlayableCharacter_C|GetElement BPC))
        (:Execute%20out
          (Utilities|StringAppend+Print "Talent : " (Utilities|String|EnumtoString (Variables|/Game/GAME/BP/Components_Interfaces/BPC_PlayableCharacter.BPC_PlayableCharacter_C|GetTalent BPC))
            (:Execute%20out
              (Utilities|StringAppend+Print "HP : " (Utilities|String|Append (Utilities|String|Append (Utilities|String|ToString(Integer) (Variables|/Game/GAME/BP/Components_Interfaces/BPC_PlayableCharacter.BPC_PlayableCharacter_C|Getcurrent%20HP BPC)) " / ") (Utilities|String|ToString(Integer) (Variables|/Game/GAME/BP/Components_Interfaces/BPC_PlayableCharacter.BPC_PlayableCharacter_C|GetBase%20HP BPC)))
                (:Execute%20out
                  (Utilities|StringAppend+Print "Level :" (Utilities|String|ToString(Integer) (Variables|/Game/GAME/BP/Components_Interfaces/BPC_PlayableCharacter.BPC_PlayableCharacter_C|GetLevel BPC))
                    (:Execute%20out
                      (Utilities|StringAppend+Print "FOR :" (Utilities|String|ToString(Integer) (Variables|/Game/GAME/BP/Components_Interfaces/BPC_PlayableCharacter.BPC_PlayableCharacter_C|GetBase%20FOR BPC))
                        (:Execute%20out
                          (Utilities|StringAppend+Print "DEF :" (Utilities|String|ToString(Integer) (Variables|/Game/GAME/BP/Components_Interfaces/BPC_PlayableCharacter.BPC_PlayableCharacter_C|GetBase%20DEF BPC))
                            (:Execute%20out
                              (Utilities|StringAppend+Print "MAG : " (Utilities|String|ToString(Integer) (Variables|/Game/GAME/BP/Components_Interfaces/BPC_PlayableCharacter.BPC_PlayableCharacter_C|GetBase%20MAG BPC))
                                (:Execute%20out
                                  (Utilities|StringAppend+Print "DEF.M :" (Utilities|String|ToString(Integer) (Variables|/Game/GAME/BP/Components_Interfaces/BPC_PlayableCharacter.BPC_PlayableCharacter_C|GetBase%20DEF_M BPC))
                                    (:Execute%20out
                                      (Utilities|StringAppend+Print "VIT :" (Utilities|String|ToString(Integer) (Variables|/Game/GAME/BP/Components_Interfaces/BPC_PlayableCharacter.BPC_PlayableCharacter_C|GetBase%20VIT BPC))
                                        (:Execute%20out
                                          (Utilities|StringAppend+Print "Ally :" (Utilities|GetDisplayName (Variables|/Game/GAME/BP/Components_Interfaces/BPC_PlayableCharacter.BPC_PlayableCharacter_C|GetAlly%20Arme%20/%20Manieur BPC))
                                            (:Execute%20out
                                              (for (_array_element _array_index) (Variables|/Game/GAME/BP/Components_Interfaces/BPC_PlayableCharacter.BPC_PlayableCharacter_C|GetUsable%20Moves BPC)
                                                (Utilities|StringAppend+Print (Utilities|String|Append (Utilities|String|Append "Move " (Utilities|String|ToString(Integer) (+ _array_index 1))) " : ") (Utilities|String|EnumtoString _array_element))))))))))))))))))))))))))

(fn UsePlayableCharacterMove
  (params (Move :type E_Moves%20Enum :default "NewEnumerator0") (BP_PlayableCharacterRef :type BP%20Playable%20Character%20in%20Battle%20Object%20Reference))
  (Utilities|PrintInfoUseMove Move BP_PlayableCharacterRef))