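; Overworld GameMode that directs Ybriss's scripted cutscenes (intro, Kento encounter, Pouloie battle lead-in), info popups and battle transitions.
; Ybriss begin either plays the intro or, if its GameInstance switch is set, restores the saved player transform.
; Cutscene beats are separate events that move the player's FreeCam between camera-root actors, animate characters and launch DataTable dialogue.
; LaunchWildBattle saves transform, level and battle info to the GameInstance, then opens the environment's battle map.
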(event Custom|LoadBattleMap
  (params (Environment :type E_Environments%20Enum :default "NewEnumerator0"))
  (Utilities|FlowControl|Delay 0.2)
  (switch Utilities|FlowControl|Switch|SwitchonE_Environments Environment
    (:NewEnumerator0
      (Game|OpenLevel(byObjectReference) "/Game/GAME/MAP/BattleMap/BMAP_YbrissDeck.BMAP_YbrissDeck"))))

(event Custom|Ybriss_Begin_Event
  (bind _as_gi_game_instance (Variables|Default|GetAs%20GI%20Game%20Instance))
  (bind _player (Variables|Default|GetPlayer))
  (bind _fadewbp (Variables|Default|GetFadeWBP))
  (bind _game_switchs (Variables|/Game/GAME/BP/General/GI_GameInstance.GI_GameInstance_C|GetGame_Switchs _as_gi_game_instance))
  (Utilities|FlowControl|Delay 0.1)
  (bind _keys (Utilities|Map|Keys _game_switchs))
  (bind _values (Utilities|Map|Values _game_switchs))
  (if (Utilities|Array|Get(acopy) _values (Utilities|Array|FindItem _keys "NewEnumerator1"))
    (Transformation|SetActorTransform _player (Variables|/Game/GAME/BP/General/GI_GameInstance.GI_GameInstance_C|GetOW_Transform _as_gi_game_instance))
    (Components|Activation|SetActive (Variables|/Game/GAME/BP/Overworld/BP_PlayerCharacter.BP_PlayerCharacter_C|GetSpringCam _player) true false)
    (Components|Animation|PlayAnimation _fadewbp (Variables|/Game/GAME/BP/Widget/WBP_Fade.WBP_Fade_C|GetFadeIn _fadewbp) 0.0 1 "Reverse"
      (:then
        (CallFunction|DestroyCinematicsBP))
      (:Finished
        (Widget|RemovefromParent _fadewbp)
        (bind _returnvalue (Audio|SpawnSound2D "/Game/GAME/AUDIO/MUSIC/First_Flight.First_Flight" 1.0 1.0 0.0 0))
        (Variables|Default|SetCurrentOST_Playing _returnvalue)))
    (else
      (CallFunction|YbrissIntroScene))))

(event Custom|FinishIntro
  (bind _player (Variables|Default|GetPlayer))
  (bind _returnvalue (UserInterface|CreateWidget "/Game/GAME/BP/Widget/WBP_Fade.WBP_Fade_C"))
  (bind _output_get (Variables|Default|SetFadeWBP _returnvalue))
  (Audio|Components|Audio|FadeOut (Variables|Default|GetCurrentOST_Playing) 0.5 0.0 "Linear" :!class /Script/Engine.AudioComponent)
  (Components|Animation|PlayAnimation _output_get (Variables|/Game/GAME/BP/Widget/WBP_Fade.WBP_Fade_C|GetFadeIn _returnvalue) 0.0
    (:then
      (UserInterface|Viewport|AddtoViewport _output_get 0))
    (:Finished
      (Utilities|FlowControl|Delay 0.2)
      (for _array_element (Utilities|Array|MakeArray "/Game/GAME/BP/Overworld/Cinematics/BP_OndeOnGround.BP_OndeOnGround_C" "/Game/GAME/BP/Overworld/Cinematics/BP_OndeSleeping.BP_OndeSleeping_C" "/Game/GAME/BP/Overworld/Cinematics/BP_Liz.BP_Liz_C" "/Game/GAME/BP/Overworld/ROOTS/BP_CamRoot_Bed.BP_CamRoot_Bed_C" "/Game/GAME/BP/Overworld/ROOTS/BP_CamRoot_Behind.BP_CamRoot_Behind_C" "/Game/GAME/BP/Overworld/ROOTS/BP_CamRoot_Entrance.BP_CamRoot_Entrance_C" "/Game/GAME/BP/Overworld/ROOTS/BP_CamRoot_FocusOnde.BP_CamRoot_FocusOnde_C")
        (bind _outactors (Actor|GetAllActorsOfClass _array_element))
        (for _array_element_2 _outactors
          (Actor|DestroyActor _array_element_2)))
      (Utilities|FlowControl|Delay 0.2)
      (Utilities|Map|Add (Variables|/Game/GAME/BP/General/GI_GameInstance.GI_GameInstance_C|GetGame_Switchs (Variables|Default|GetAs%20GI%20Game%20Instance)) "NewEnumerator1" true)
      (Variables|/Game/GAME/BP/Overworld/BP_PlayerCharacter.BP_PlayerCharacter_C|SetCanMove? _player true)
      (Variables|/Game/GAME/BP/Overworld/BP_PlayerCharacter.BP_PlayerCharacter_C|SetCanInteract? _player true)
      (Variables|/Game/GAME/BP/Overworld/BP_PlayerCharacter.BP_PlayerCharacter_C|SetIsFreeCam? _player false)
      (Components|Activation|Deactivate (Variables|/Game/GAME/BP/Overworld/BP_PlayerCharacter.BP_PlayerCharacter_C|GetFreeCam _player))
      (Components|Activation|Activate (Variables|/Game/GAME/BP/Overworld/BP_PlayerCharacter.BP_PlayerCharacter_C|GetSpringCam _player) true)
      (Rendering|SetActorHiddenInGame _player false)
      (Components|Animation|PlayAnimation _output_get (Variables|/Game/GAME/BP/Widget/WBP_Fade.WBP_Fade_C|GetFadeIn _returnvalue) 0.0 1 "Reverse"
        (:Finished
          (Widget|RemovefromParent _output_get)
          (bind _returnvalue_2 (Audio|SpawnSound2D "/Game/GAME/AUDIO/MUSIC/First_Flight.First_Flight" 1.0 1.0 0.0 0))
          (Variables|Default|SetCurrentOST_Playing _returnvalue_2))))))

(event Custom|KentoRencontre
  (params (FadeWBP :type WBP%20Fade%20Object%20Reference))
  (Variables|/Game/GAME/BP/Components_Interfaces/BPC_Dialogue.BPC_Dialogue_C|SetPlayer (Variables|Default|GetBPC_Dialogue) (Variables|Default|GetPlayer))
  (Input|EnableInput (Variables|Default|GetPlayer) 0)
  (Development|PrintString "event proc")
  (Variables|/Game/GAME/BP/Overworld/BP_PlayerCharacter.BP_PlayerCharacter_C|SetCanInteract? (Variables|Default|GetPlayer) false)
  (Variables|/Game/GAME/BP/Overworld/BP_PlayerCharacter.BP_PlayerCharacter_C|SetCanMove? (Variables|Default|GetPlayer) false)
  (Variables|/Game/GAME/BP/Overworld/BP_PlayerCharacter.BP_PlayerCharacter_C|SetIsFreeCam? (Variables|Default|GetPlayer) true)
  (Components|Activation|Deactivate (Variables|/Game/GAME/BP/Overworld/BP_PlayerCharacter.BP_PlayerCharacter_C|GetSpringCam (Variables|Default|GetPlayer)))
  (Components|Activation|Activate (Variables|/Game/GAME/BP/Overworld/BP_PlayerCharacter.BP_PlayerCharacter_C|GetFreeCam (Variables|Default|GetPlayer)) false)
  (Rendering|SetActorHiddenInGame (Variables|Default|GetPlayer) true)
  (Transformation|SetWorldTransform (Variables|/Game/GAME/BP/Overworld/BP_PlayerCharacter.BP_PlayerCharacter_C|GetFreeCam (Variables|Default|GetPlayer)) (CallFunction|GetCamTransform "/Game/GAME/BP/Overworld/ROOTS/BP_CamRoot_FirstKento.BP_CamRoot_FirstKento_C") false false)
  (bind _outactors (Actor|GetAllActorsOfClass "/Game/GAME/BP/Overworld/Cinematics/BP_OndeSearching.BP_OndeSearching_C"))
  (Rendering|SetActorHiddenInGame (Utilities|Array|Get(acopy) _outactors) false)
  (Components|Animation|PlayAnimation (Variables|/Game/GAME/BP/Overworld/Cinematics/BP_OndeSearching.BP_OndeSearching_C|GetSkeletalMesh (Utilities|Array|Get(acopy) _outactors)) "/Game/GAME/ASSETS/3D/CHARACTERS/ONDE/ANIM/Looking_Around.Looking_Around" false)
  (Components|Animation|PlayAnimation FadeWBP (Variables|/Game/GAME/BP/Widget/WBP_Fade.WBP_Fade_C|GetFadeIn FadeWBP) 0.0 1 "Reverse"
    (:then
      (Utilities|FlowControl|Delay 6.0)
      (CallFunction|KentoTurnAround))
    (:Finished
      (Widget|RemovefromParent FadeWBP)
      (Development|PrintString "fini"))))

(event Custom|KentoTurnAround
  (bind _outactors (Actor|GetAllActorsOfClass "/Game/GAME/BP/Overworld/Cinematics/BP_Kento.BP_Kento_C"))
  (Rendering|SetActorHiddenInGame (Utilities|Array|Get(acopy) _outactors) false)
  (Transformation|SetWorldTransform (Variables|/Game/GAME/BP/Overworld/BP_PlayerCharacter.BP_PlayerCharacter_C|GetFreeCam (Variables|Default|GetPlayer)) (CallFunction|GetCamTransform "/Game/GAME/BP/Overworld/ROOTS/BP_CamRoot_KentoFocus.BP_CamRoot_KentoFocus_C") false true)
  (Variables|Default|SetAimRot (Math|Rotator|MakeRotator (.Roll (Math|Rotator|BreakRotator (Transformation|GetWorldRotation (Variables|/Game/GAME/BP/Overworld/Cinematics/BP_Kento.BP_Kento_C|GetDefaultSceneRoot (Utilities|Array|Get(acopy) _outactors))))) (.Pitch (Math|Rotator|BreakRotator (Transformation|GetWorldRotation (Variables|/Game/GAME/BP/Overworld/Cinematics/BP_Kento.BP_Kento_C|GetDefaultSceneRoot (Utilities|Array|Get(acopy) _outactors))))) (+ (.Yaw (Math|Rotator|BreakRotator (Transformation|GetWorldRotation (Variables|/Game/GAME/BP/Overworld/Cinematics/BP_Kento.BP_Kento_C|GetDefaultSceneRoot (Utilities|Array|Get(acopy) _outactors))))) 1.8e+02)))
  (Components|Animation|PlayAnimation (Variables|/Game/GAME/BP/Overworld/Cinematics/BP_Kento.BP_Kento_C|GetSkeletalMesh (Utilities|Array|Get(acopy) _outactors)) "/Game/GAME/ASSETS/3D/CHARACTERS/MATELOT/Walking.Walking" true)
  (bind _newtrack_0 (Timeline|Timeline PlayFromStart)
    (:Update
      (Transformation|SetWorldRotation (Variables|/Game/GAME/BP/Overworld/Cinematics/BP_Kento.BP_Kento_C|GetDefaultSceneRoot (Utilities|Array|Get(acopy) _outactors)) (Math|Rotator|MakeRotator (.roll (Variables|Default|GetAimRot)) (.pitch (Variables|Default|GetAimRot)) (.yaw (Math|Rotator|Lerp(Rotator) (Transformation|GetWorldRotation (Variables|/Game/GAME/BP/Overworld/Cinematics/BP_Kento.BP_Kento_C|GetDefaultSceneRoot (Utilities|Array|Get(acopy) _outactors))) (Variables|Default|GetAimRot) _newtrack_0))) false false))
    (:Finished
      (Default|LaunchDialogue (Variables|Default|GetBPC_Dialogue) "/Game/GAME/DATA/DATA_TABLE/Dialogues/DT_KentoEncounter.DT_KentoEncounter" 1)
      (Components|Animation|PlayAnimation (Variables|/Game/GAME/BP/Overworld/Cinematics/BP_Kento.BP_Kento_C|GetSkeletalMesh (Utilities|Array|Get(acopy) _outactors)) "/Game/GAME/ASSETS/3D/CHARACTERS/MATELOT/Breathing_Idle__1_.Breathing_Idle__1_" true))))

(event Custom|Onde%20Approaching
  (bind _outactors (Actor|GetAllActorsOfClass "/Game/GAME/BP/Overworld/Cinematics/BP_OndeSearching.BP_OndeSearching_C"))
  (Components|Animation|PlayAnimation (Variables|/Game/GAME/BP/Overworld/Cinematics/BP_OndeSearching.BP_OndeSearching_C|GetSkeletalMesh (Utilities|Array|Get(acopy) _outactors)) "/Game/GAME/ASSETS/3D/CHARACTERS/ONDE/ANIM/Standard_Run.Standard_Run" true)
  (bind _outactors_2 (Actor|GetAllActorsOfClass "/Game/GAME/BP/Overworld/ROOTS/BP_RootsCloseToKento.BP_RootsCloseToKento_C"))
  (Variables|Default|SetAimLocation (Math|Transform|MakeTransform (.location (Transformation|GetActorTransform (Utilities|Array|Get(acopy) _outactors_2))) (.rotation (Transformation|GetActorTransform (Utilities|Array|Get(acopy) _outactors))) (.scale (Transformation|GetActorTransform (Utilities|Array|Get(acopy) _outactors)))))
  (Transformation|SetWorldTransform (Variables|/Game/GAME/BP/Overworld/BP_PlayerCharacter.BP_PlayerCharacter_C|GetFreeCam (Variables|Default|GetPlayer)) (CallFunction|GetCamTransform "/Game/GAME/BP/Overworld/ROOTS/BP_CamRoot_Approaching.BP_CamRoot_Approaching_C") false false)
  (Timeline|Timeline_0 PlayFromStart
    (:Update
      (Transformation|SetActorTransform (Utilities|Array|Get(acopy) _outactors) (Math|Transform|MakeTransform (+ (.location (Transformation|GetActorTransform (Utilities|Array|Get(acopy) _outactors))) (* (Math|Vector|Normalize (- (.location (Variables|Default|GetAimLocation)) (.location (Transformation|GetActorTransform (Utilities|Array|Get(acopy) _outactors))))) 1e+01)) (.rotation (Transformation|GetActorTransform (Utilities|Array|Get(acopy) _outactors))) (.scale (Transformation|GetActorTransform (Utilities|Array|Get(acopy) _outactors))))))
    (:Finished
      (Components|Animation|PlayAnimation (Variables|/Game/GAME/BP/Overworld/Cinematics/BP_OndeSearching.BP_OndeSearching_C|GetSkeletalMesh (Utilities|Array|Get(acopy) _outactors)) "/Game/GAME/ASSETS/3D/CHARACTERS/ONDE/ANIM/Idle__1_.Idle__1_" true)
      (CallFunction|KentoCloseDialogue))))

(event Custom|Ondefocus
  (bind _outactors (Actor|GetAllActorsOfClass "/Game/GAME/BP/Overworld/Cinematics/BP_OndeSearching.BP_OndeSearching_C"))
  (Components|Animation|PlayAnimation (Variables|/Game/GAME/BP/Overworld/Cinematics/BP_OndeSearching.BP_OndeSearching_C|GetSkeletalMesh (Utilities|Array|Get(acopy) _outactors)) "/Game/GAME/ASSETS/3D/CHARACTERS/ONDE/ANIM/Idle__1_.Idle__1_" false)
  (Transformation|SetWorldTransform (Variables|/Game/GAME/BP/Overworld/BP_PlayerCharacter.BP_PlayerCharacter_C|GetFreeCam (Variables|Default|GetPlayer)) (CallFunction|GetCamTransform "/Game/GAME/BP/Overworld/ROOTS/BP_CamRoot_FirstKento.BP_CamRoot_FirstKento_C") false false))

(event Custom|KentoFocus
  (Transformation|SetWorldTransform (Variables|/Game/GAME/BP/Overworld/BP_PlayerCharacter.BP_PlayerCharacter_C|GetFreeCam (Variables|Default|GetPlayer)) (CallFunction|GetCamTransform "/Game/GAME/BP/Overworld/ROOTS/BP_CamRoot_KentoFocus.BP_CamRoot_KentoFocus_C") false true))

(event Custom|KentoCloseDialogue
  (Default|LaunchDialogue (Variables|Default|GetBPC_Dialogue) "/Game/GAME/DATA/DATA_TABLE/Dialogues/DT_KentoEncounter.DT_KentoEncounter" 8))

(event Custom|OndeNotShocked
  (bind _outactors (Actor|GetAllActorsOfClass "/Game/GAME/BP/Overworld/Cinematics/BP_OndeSearching.BP_OndeSearching_C"))
  (Rendering|Material|SetMaterial (Variables|/Game/GAME/BP/Overworld/Cinematics/BP_OndeSearching.BP_OndeSearching_C|GetSkeletalMesh (Utilities|Array|Get(acopy) _outactors)) 0 "/Game/GAME/ASSETS/3D/CHARACTERS/ONDE/Textures/T_face.T_face")
  (Utilities|FlowControl|Delay 0.2)
  (Transformation|SetWorldTransform (Variables|/Game/GAME/BP/Overworld/BP_PlayerCharacter.BP_PlayerCharacter_C|GetFreeCam (Variables|Default|GetPlayer)) (CallFunction|GetCamTransform "/Game/GAME/BP/Overworld/ROOTS/BP_CamRoot_Ondeshocked.BP_CamRoot_Ondeshocked_C") false true))

(event Custom|OndeShocked
  (bind _outactors (Actor|GetAllActorsOfClass "/Game/GAME/BP/Overworld/Cinematics/BP_OndeSearching.BP_OndeSearching_C"))
  (Rendering|Material|SetMaterial (Variables|/Game/GAME/BP/Overworld/Cinematics/BP_OndeSearching.BP_OndeSearching_C|GetSkeletalMesh (Utilities|Array|Get(acopy) _outactors)) 0 "/Game/GAME/ASSETS/3D/CHARACTERS/ONDE/Textures/T_onde_shocked/MI_OndeShocked.MI_OndeShocked")
  (Utilities|FlowControl|Delay 0.5)
  (Transformation|SetWorldTransform (Variables|/Game/GAME/BP/Overworld/BP_PlayerCharacter.BP_PlayerCharacter_C|GetFreeCam (Variables|Default|GetPlayer)) (CallFunction|GetCamTransform "/Game/GAME/BP/Overworld/ROOTS/BP_CamRoot_Ondeshocked.BP_CamRoot_Ondeshocked_C") false true)
  (Default|LaunchDialogue (Variables|Default|GetBPC_Dialogue) "/Game/GAME/DATA/DATA_TABLE/Dialogues/DT_KentoEncounter.DT_KentoEncounter" 11))

(event Custom|ShowInfoText
  (params (Text :type String))
  (bind _player (Variables|Default|GetPlayer))
  (Variables|/Game/GAME/BP/Overworld/BP_PlayerCharacter.BP_PlayerCharacter_C|SetCanInteract? _player false)
  (Variables|/Game/GAME/BP/Overworld/BP_PlayerCharacter.BP_PlayerCharacter_C|SetCanMove? _player false)
  (Variables|/Game/GAME/BP/Overworld/BP_PlayerCharacter.BP_PlayerCharacter_C|SetIsInInfo? _player true)
  (bind _returnvalue (UserInterface|CreateWidget "/Game/GAME/BP/Widget/WBP_Info.WBP_Info_C"))
  (bind _output_get (Variables|Default|SetWBP _returnvalue))
  (Variables|/Game/GAME/BP/Widget/WBP_Info.WBP_Info_C|SetGM_Ref _output_get self)
  (UserInterface|Viewport|AddtoViewport _output_get 0)
  (Default|TypeWritter _output_get Text 0.04))

(event Custom|PouloieEvent
  (bind _player (Variables|Default|GetPlayer))
  (bind _freecam (Variables|/Game/GAME/BP/Overworld/BP_PlayerCharacter.BP_PlayerCharacter_C|GetFreeCam _player))
  (Transformation|SetWorldTransform _freecam (CallFunction|GetCamTransform "/Game/GAME/BP/Overworld/ROOTS/BP_CamRoot_LargePouloie.BP_CamRoot_LargePouloie_C") false false)
  (Audio|PlaySound2D "/Game/GAME/AUDIO/SE/Mobs/Pouloie.Pouloie" 5.0 1.0 0.0 0 0)
  (Utilities|FlowControl|Delay 0.2)
  (Utilities|FlowControl|Sequence
    (:then_0
      (Utilities|FlowControl|Delay 1.2)
      (Default|LaunchDialogue (Variables|Default|GetBPC_Dialogue) "/Game/GAME/DATA/DATA_TABLE/Dialogues/DT_KentoEncounter.DT_KentoEncounter" 19))
    (:then_1
      (Audio|PlaySound2D "/Game/GAME/AUDIO/SE/Cinematics/Medium_Impact.Medium_Impact" 1.0 1.0 0.0 0 0)
      (Camera|PlayWorldCameraShake "/Game/GAME/BP/General/Shakes/BP_CamShake_Pouloie.BP_CamShake_Pouloie_C" (Transformation|GetWorldLocation _freecam) 0.0 1e+03))
    (:then_2
      (Utilities|FlowControl|Delay 0.2)
      (Audio|PlaySound2D "/Game/GAME/AUDIO/SE/Cinematics/Medium_Impact.Medium_Impact" 1.2 1.0 0.0 0 0)
      (Camera|PlayWorldCameraShake "/Game/GAME/BP/General/Shakes/BP_CamShake_Pouloie.BP_CamShake_Pouloie_C" "0, 0, 0" 0.0 1e+03))
    (:then_3
      (Utilities|FlowControl|Delay 0.3)
      (Audio|PlaySound2D "/Game/GAME/AUDIO/SE/Cinematics/Medium_Impact.Medium_Impact" 1.0 1.0 0.0 0 0)
      (Camera|PlayWorldCameraShake "/Game/GAME/BP/General/Shakes/BP_CamShake_Pouloie.BP_CamShake_Pouloie_C" "0, 0, 0" 0.0 1e+03))))

(event Custom|PouloieExit
  (bind _returnvalue (UserInterface|CreateWidget "/Game/GAME/BP/Widget/WBP_Fade.WBP_Fade_C"))
  (Components|Animation|PlayAnimation _returnvalue (Variables|/Game/GAME/BP/Widget/WBP_Fade.WBP_Fade_C|GetFadeIn _returnvalue) 0.0
    (:then
      (UserInterface|Viewport|AddtoViewport _returnvalue 0))
    (:Finished
      (bind _outactors (Actor|GetAllActorsOfClass "/Game/GAME/BP/Overworld/Cinematics/BP_Pouloie.BP_Pouloie_C"))
      (for _array_element _outactors
        (Rendering|SetActorHiddenInGame _array_element false))
      (bind _outactors_2 (Actor|GetAllActorsOfClass "/Game/GAME/BP/Overworld/Cinematics/BP_Rahf.BP_Rahf_C"))
      (Rendering|SetActorHiddenInGame (Utilities|Array|Get(acopy) _outactors_2) false)
      (Transformation|SetWorldTransform (Variables|/Game/GAME/BP/Overworld/BP_PlayerCharacter.BP_PlayerCharacter_C|GetFreeCam (Variables|Default|GetPlayer)) (CallFunction|GetCamTransform "/Game/GAME/BP/Overworld/ROOTS/BP_Cam_Pouloie.BP_Cam_Pouloie_C") false false)
      (Components|Animation|PlayAnimation _returnvalue (Variables|/Game/GAME/BP/Widget/WBP_Fade.WBP_Fade_C|GetFadeIn _returnvalue) 0.0 1 "Reverse"
        (:Finished
          (Widget|RemovefromParent _returnvalue)
          (Default|LaunchDialogue (Variables|Default|GetBPC_Dialogue) "/Game/GAME/DATA/DATA_TABLE/Dialogues/DT_KentoEncounter.DT_KentoEncounter" 21))))))

(event Custom|GoFacePouloie
  (bind _as_gi_game_instance (Variables|Default|GetAs%20GI%20Game%20Instance))
  (bind _output_get (Variables|/Game/GAME/BP/General/GI_GameInstance.GI_GameInstance_C|SetBaseTeam _as_gi_game_instance (Variables|/Game/GAME/BP/General/GI_GameInstance.GI_GameInstance_C|GetPlayerTeam _as_gi_game_instance)))
  (bind _output_get_2 (Variables|/Game/GAME/BP/General/GI_GameInstance.GI_GameInstance_C|SetPlayerTeam _as_gi_game_instance _output_get))
  (Utilities|Array|Add _output_get_2 (Utilities|Struct|MakeST_PlayerTeam "NewEnumerator2" 50 0 0 0 0 0))
  (Transformation|SetWorldTransform (Variables|/Game/GAME/BP/Overworld/BP_PlayerCharacter.BP_PlayerCharacter_C|GetFreeCam (Variables|Default|GetPlayer)) (CallFunction|GetCamTransform "/Game/GAME/BP/Overworld/ROOTS/BP_Cam_Pouloie.BP_Cam_Pouloie_C") false false)
  (bind _outactors (Actor|GetAllActorsOfClass "/Game/GAME/BP/Overworld/Cinematics/BP_Pouloie.BP_Pouloie_C"))
  (for _array_element _outactors
    (Components|Animation|PlayAnimation (Variables|/Game/GAME/BP/Overworld/Cinematics/BP_Pouloie.BP_Pouloie_C|GetSkeletalMesh _array_element) "/Game/GAME/ASSETS/3D/MOBS/New_Pouloie/ANIMS/Pouloie2_Anim_Armature_ATTACK_M.Pouloie2_Anim_Armature_ATTACK_M" false))
  (Utilities|FlowControl|Delay 0.5)
  (Audio|PlaySound2D "/Game/GAME/AUDIO/SE/Mobs/Pouloie.Pouloie" 3.0 1.0 0.0 0 0)
  (Utilities|FlowControl|Delay 0.2)
  (Default|LaunchBattle (Variables|Default|GetPlayer) 1 "/Game/GAME/DATA/DATA_TABLE/Battles/DT_YbrissBattle.DT_YbrissBattle"))

(event Custom|Ybriss_Intro_Scene
  (bind _bpc_dialogue (Variables|Default|GetBPC_Dialogue))
  (bind _fadewbp (Variables|Default|GetFadeWBP))
  (bind _as_gi_game_instance (Variables|Default|GetAs%20GI%20Game%20Instance))
  (bind _playerteam (Variables|/Game/GAME/BP/General/GI_GameInstance.GI_GameInstance_C|GetPlayerTeam _as_gi_game_instance))
  (Utilities|Array|Clear _playerteam)
  (Utilities|Array|SetArrayElem _playerteam 0 (Utilities|Struct|MakeST_PlayerTeam "NewEnumerator0" 5 0 0 0 0 10))
  (Rendering|SetActorHiddenInGame (Variables|Default|GetPlayer) true)
  (bind _returnvalue (Audio|SpawnSound2D "/Game/GAME/AUDIO/MUSIC/Strange_Theme.Strange_Theme" 0.7 1.0 0.0 0))
  (Variables|Default|SetCurrentOST_Playing _returnvalue)
  (Class|GameplayStatics|LoadStreamLevelbySoftObjectPtr "/Game/GAME/MAP/SUBLEVELS/Map0_Inside.Map0_Inside" true false)
  (bind _outactors (Actor|GetAllActorsOfClass "/Game/GAME/BP/Overworld/ROOTS/BP_BedRoot.BP_BedRoot_C"))
  (Variables|/Game/GAME/BP/Overworld/BP_PlayerCharacter.BP_PlayerCharacter_C|SetCanMove? (Variables|Default|GetPlayer) false)
  (Variables|/Game/GAME/BP/Overworld/BP_PlayerCharacter.BP_PlayerCharacter_C|SetCanInteract? (Variables|Default|GetPlayer) false)
  (Variables|/Game/GAME/BP/Overworld/BP_PlayerCharacter.BP_PlayerCharacter_C|SetIsFreeCam? (Variables|Default|GetPlayer) true)
  (bind _outactors_2 (Actor|GetAllActorsOfClass "/Game/GAME/BP/Overworld/ROOTS/BP_CamRoot_Bed.BP_CamRoot_Bed_C"))
  (Utilities|IsValid (Utilities|Array|Get(acopy) _outactors_2)
    (:Is%20Valid
      (Components|Activation|SetActive (Variables|/Game/GAME/BP/Overworld/BP_PlayerCharacter.BP_PlayerCharacter_C|GetFreeCam (Variables|Default|GetPlayer)) true false)
      (Transformation|SetActorLocation (Variables|Default|GetPlayer) (Transformation|GetActorLocation (Utilities|Array|Get(acopy) _outactors)) false false)
      (Transformation|SetWorldTransform (Variables|/Game/GAME/BP/Overworld/BP_PlayerCharacter.BP_PlayerCharacter_C|GetFreeCam (Variables|Default|GetPlayer)) (Transformation|GetWorldTransform (Variables|/Game/GAME/BP/Overworld/ROOTS/BP_CamRoot_Bed.BP_CamRoot_Bed_C|GetCamera (Utilities|Array|Get(acopy) _outactors_2))) false true)
      (Components|Animation|PlayAnimation _fadewbp (Variables|/Game/GAME/BP/Widget/WBP_Fade.WBP_Fade_C|GetFadeIn _fadewbp) 0.0 1 "Reverse"
        (:then
          (Variables|/Game/GAME/BP/Components_Interfaces/BPC_Dialogue.BPC_Dialogue_C|SetPlayer _bpc_dialogue (Variables|Default|GetPlayer))
          (Default|LaunchDialogue _bpc_dialogue "/Game/GAME/DATA/DATA_TABLE/Dialogues/DT_IntroDialogue.DT_IntroDialogue" 1))
        (:Finished
          (Widget|RemovefromParent _fadewbp))))))

(event Custom|OndeFalls
  (Utilities|FlowControl|Delay 0.5)
  (Audio|PlaySound2D "/Game/GAME/AUDIO/SE/Cinematics/Onde_Impact.Onde_Impact" 1.0 0.7 0.0 0 0)
  (Camera|PlayWorldCameraShake "/Game/GAME/BP/General/Shakes/BP_CamShakeDamage.BP_CamShakeDamage_C" (.Location (Math|Transform|BreakTransform (Transformation|GetWorldTransform (Variables|/Game/GAME/BP/Overworld/ROOTS/BP_CamRoot.BP_CamRoot_C|GetCamera (Utilities|Array|Get(acopy) (stale Custom|LizEnters _outactors)))))) 0.0 1e+03)
  (Utilities|FlowControl|Delay 0.75)
  (Default|LaunchDialogue (Variables|Default|GetBPC_Dialogue) "/Game/GAME/DATA/DATA_TABLE/Dialogues/DT_IntroDialogue.DT_IntroDialogue" 5))

(event Custom|LizEnters
  (bind _outactors (Actor|GetAllActorsOfClass "/Game/GAME/BP/Overworld/ROOTS/BP_CamRoot_Entrance.BP_CamRoot_Entrance_C"))
  (Transformation|SetWorldTransform (Variables|/Game/GAME/BP/Overworld/BP_PlayerCharacter.BP_PlayerCharacter_C|GetFreeCam (Variables|Default|GetPlayer)) (Transformation|GetWorldTransform (Variables|/Game/GAME/BP/Overworld/ROOTS/BP_CamRoot.BP_CamRoot_C|GetCamera (Utilities|Array|Get(acopy) _outactors))) false false)
  (Audio|PlaySound2D "/Game/GAME/AUDIO/SE/Environment/Closing_Door.Closing_Door" 1.0 1.0 0.0 0 0)
  (Utilities|FlowControl|Delay 1.5)
  (bind _outactors_2 (Actor|GetAllActorsOfClass "/Game/GAME/BP/Overworld/Cinematics/BP_Liz.BP_Liz_C"))
  (Components|Animation|PlayAnimation (Variables|/Game/GAME/BP/Overworld/Cinematics/BP_Liz.BP_Liz_C|GetSkeletalMesh (Utilities|Array|Get(acopy) _outactors_2)) "/Game/GAME/ASSETS/3D/CHARACTERS/MATELOTTE/Yelling_While_Standing.Yelling_While_Standing" false)
  (Utilities|FlowControl|Sequence
    (:then_0
      (Default|LaunchDialogue (Variables|Default|GetBPC_Dialogue) "/Game/GAME/DATA/DATA_TABLE/Dialogues/DT_IntroDialogue.DT_IntroDialogue" 4)
      (Utilities|FlowControl|Delay 0.5)
      (Camera|PlayWorldCameraShake "/Game/GAME/BP/General/Shakes/BP_CamShakeLizYell.BP_CamShakeLizYell_C" (.Location (Math|Transform|BreakTransform (Transformation|GetWorldTransform (Variables|/Game/GAME/BP/Overworld/ROOTS/BP_CamRoot.BP_CamRoot_C|GetCamera (Utilities|Array|Get(acopy) _outactors))))) 0.0 1e+03))
    (:then_1
      (Utilities|FlowControl|Delay 2.5)
      (Components|Animation|PlayAnimation (Variables|/Game/GAME/BP/Overworld/Cinematics/BP_Liz.BP_Liz_C|GetSkeletalMesh (Utilities|Array|Get(acopy) _outactors_2)) "/Game/GAME/ASSETS/3D/CHARACTERS/MATELOTTE/Idle.Idle" true))))

(event Custom|CloseInfo
  (Widget|RemovefromParent (Variables|Default|GetWBP)))

(event Custom|DestroyCinematicsBP
  (for _array_element (Variables|Default|GetBP_CinematicsClass)
    (bind _outactors (Actor|GetAllActorsOfClass _array_element))
    (for _array_element_2 _outactors
      (Actor|DestroyActor _array_element_2))))

(event Custom|OndeGetUp
  (bind _outactors (Actor|GetAllActorsOfClass "/Game/GAME/BP/Overworld/Cinematics/BP_OndeSleeping.BP_OndeSleeping_C"))
  (Rendering|SetActorHiddenInGame (Utilities|Array|Get(acopy) _outactors) true)
  (bind _outactors_2 (Actor|GetAllActorsOfClass "/Game/GAME/BP/Overworld/Cinematics/BP_OndeOnGround.BP_OndeOnGround_C"))
  (Rendering|SetActorHiddenInGame (Utilities|Array|Get(acopy) _outactors_2) false)
  (Components|Animation|PlayAnimation (Variables|/Game/GAME/BP/Overworld/Cinematics/BP_OndeOnGround.BP_OndeOnGround_C|GetSkeletalMesh (Utilities|Array|Get(acopy) _outactors_2)) "/Game/GAME/ASSETS/3D/CHARACTERS/ONDE/ANIM/Standing_Up__2_.Standing_Up__2_" false)
  (Utilities|FlowControl|Sequence
    (:then_0
      (bind _outactors_3 (Actor|GetAllActorsOfClass "/Game/GAME/BP/Overworld/ROOTS/BP_CamRoot_Behind.BP_CamRoot_Behind_C"))
      (Transformation|SetWorldTransform (Variables|/Game/GAME/BP/Overworld/BP_PlayerCharacter.BP_PlayerCharacter_C|GetFreeCam (Variables|Default|GetPlayer)) (Transformation|GetWorldTransform (Variables|/Game/GAME/BP/Overworld/ROOTS/BP_CamRoot.BP_CamRoot_C|GetCamera (Utilities|Array|Get(acopy) _outactors_3))) false true)
      (Utilities|FlowControl|Delay 0.5)
      (Default|LaunchDialogue (Variables|Default|GetBPC_Dialogue) "/Game/GAME/DATA/DATA_TABLE/Dialogues/DT_IntroDialogue.DT_IntroDialogue" 6))
    (:then_1
      (Utilities|FlowControl|Delay 6.2)
      (Components|Animation|PlayAnimation (Variables|/Game/GAME/BP/Overworld/Cinematics/BP_OndeOnGround.BP_OndeOnGround_C|GetSkeletalMesh (Utilities|Array|Get(acopy) _outactors_2)) "/Game/GAME/ASSETS/3D/CHARACTERS/ONDE/ANIM/Idle__1_.Idle__1_" true))))

(event Custom|LizLeaving
  (Utilities|FlowControl|Delay 0.2)
  (bind _outactors (Actor|GetAllActorsOfClass "/Game/GAME/BP/Overworld/ROOTS/BP_CamRoot_FocusOnde.BP_CamRoot_FocusOnde_C"))
  (Transformation|SetWorldTransform (Variables|/Game/GAME/BP/Overworld/BP_PlayerCharacter.BP_PlayerCharacter_C|GetFreeCam (Variables|Default|GetPlayer)) (Transformation|GetWorldTransform (Variables|/Game/GAME/BP/Overworld/ROOTS/BP_CamRoot.BP_CamRoot_C|GetCamera (Utilities|Array|Get(acopy) _outactors))) false true)
  (Audio|PlaySound2D "/Game/GAME/AUDIO/SE/Environment/Opening_Door.Opening_Door" 1.0 1.0 0.0 0 0)
  (Utilities|FlowControl|Sequence
    (:then_0
      (Utilities|FlowControl|Delay 1.5)
      (bind _outactors_2 (Actor|GetAllActorsOfClass "/Game/GAME/BP/Overworld/Cinematics/BP_OndeOnGround.BP_OndeOnGround_C"))
      (Rendering|Material|SetMaterial (Variables|/Game/GAME/BP/Overworld/Cinematics/BP_OndeOnGround.BP_OndeOnGround_C|GetSkeletalMesh (Utilities|Array|Get(acopy) _outactors_2)) 0 "/Game/GAME/ASSETS/3D/CHARACTERS/ONDE/Textures/T_face.T_face")
      (Default|LaunchDialogue (Variables|Default|GetBPC_Dialogue) "/Game/GAME/DATA/DATA_TABLE/Dialogues/DT_IntroDialogue.DT_IntroDialogue" 10))
    (:then_1
      (Utilities|FlowControl|Delay 0.6)
      (Audio|PlaySound2D "/Game/GAME/AUDIO/SE/Environment/Closing_Door.Closing_Door" 1.0 1.0 0.0 0 0))))

(event EventBeginPlay
  (bind _asgi_game_instance (Utilities|Casting|CastToGI_GameInstance (Game|GetGameInstance)))
  (bind _output_get (Variables|Default|SetAs%20GI%20Game%20Instance _asgi_game_instance))
  (bind _returnvalue (UserInterface|CreateWidget "/Game/GAME/BP/Widget/WBP_Fade.WBP_Fade_C"))
  (bind _output_get_2 (Variables|Default|SetFadeWBP _returnvalue))
  (UserInterface|Viewport|AddtoViewport _output_get_2 0)
  (Utilities|FlowControl|Delay 0.1)
  (if (Variables|/Game/GAME/BP/General/GI_GameInstance.GI_GameInstance_C|GetisInmainMenu _output_get)
    (Widget|RemovefromParent _output_get_2)))

(event EventTick
  (params (DeltaSeconds :type Float%20%28single-precision%29)))

(fn ConstructionScript)

(fn LaunchWildBattle
  (params (DataTableRef :type Data%20Table%20Object%20Reference) (RowNumber :type Integer))
  (bind _as_gi_game_instance (Variables|Default|GetAs%20GI%20Game%20Instance))
  (Variables|/Game/GAME/BP/General/GI_GameInstance.GI_GameInstance_C|SetOW_Transform _as_gi_game_instance (Transformation|GetActorTransform (Game|Player|GetPlayerPawn 0)))
  (bind _returnvalue (Game|GetCurrentLevelName true))
  (Variables|/Game/GAME/BP/General/GI_GameInstance.GI_GameInstance_C|SetCurrentLevel _as_gi_game_instance _returnvalue)
  (bind _returnvalue_2 (Utilities|GetDataTableRow DataTableRef (Utilities|String|StringToName (Utilities|String|ToString(Integer) RowNumber)))
    (:then
      (Default|SetBattleInfo _as_gi_game_instance RowNumber DataTableRef)
      (CallFunction|LoadBattleMap (.Environment (Utilities|Struct|BreakST_WildBattle _returnvalue_2))))))

(fn GetCamTransform
  (params (CamRoot :type BP%20Cam%20Root%20Class%20Reference))
  (bind _outactors (Actor|GetAllActorsOfClass CamRoot))
  (return (Transformation|GetWorldTransform (Variables|/Game/GAME/BP/Overworld/ROOTS/BP_CamRoot.BP_CamRoot_C|GetCamera (Utilities|Array|Get(acopy) _outactors)))))