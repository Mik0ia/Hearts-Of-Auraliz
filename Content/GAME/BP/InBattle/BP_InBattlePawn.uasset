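; Player pawn for battles that creates the battle HUD and turns Enhanced Input presses into menu choices.
; Boolean flags form the menu state: X, Y and A toggle Manieur move, Arme move or item selection.
; X and Y swap the current character to its Manieur or Arme ally as needed.
; In move selection, A sends the move at MenuIndex to GM_BattleGameMode; item selection only prints debug text.
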(event Input|EnhancedActionEvents|EnhancedInputActionIA_DebugButton
  (params (ActionValue :type Boolean) (ElapsedSeconds :type Float%20%28double-precision%29) (TriggeredSeconds :type Float%20%28double-precision%29) (InputAction :type Input%20Action%20Object%20Reference :default "/Game/GAME/INPUT/Actions/IA_DebugButton.IA_DebugButton"))
  (:Started
    (Development|PrintString (Utilities|GetDisplayName (Variables|Default|GetCurrentCharacter)))))

(event Input|EnhancedActionEvents|EnhancedInputActionIA_X_InBattle
  (params (ActionValue :type Boolean) (ElapsedSeconds :type Float%20%28double-precision%29) (TriggeredSeconds :type Float%20%28double-precision%29) (InputAction :type Input%20Action%20Object%20Reference :default "/Game/GAME/INPUT/Actions/InBattle/IA_X_InBattle.IA_X_InBattle"))
  (:Started
    (if (Variables|Default|GetIsChoosingAction?)
      (Variables|Default|SetIsChoosingAction? false)
      (Variables|Default|SetIsChoosingManieurMove? true)
      (if (Variables|/Game/GAME/BP/Components/BPC_PlayableCharacter.BPC_PlayableCharacter_C|GetIsManieur? (Variables|/Game/GAME/BP/InBattle/Manieur_Armes/BP_PlayableCharacterInBattle.BP_PlayableCharacterInBattle_C|GetBPC_PlayableCharacter (Variables|Default|GetCurrentCharacter)))
        _
        (else
          (Variables|Default|SetCurrentCharacter (Variables|/Game/GAME/BP/Components/BPC_PlayableCharacter.BPC_PlayableCharacter_C|GetAlly%20Arme%20/%20Manieur (Variables|/Game/GAME/BP/InBattle/Manieur_Armes/BP_PlayableCharacterInBattle.BP_PlayableCharacterInBattle_C|GetBPC_PlayableCharacter (Variables|Default|GetCurrentCharacter))))))
      (Development|PrintString "choose Manieur Move" true true "(R=0.000000,G=0.453341,B=1.000000,A=1.000000)")
      (elif (Variables|Default|GetIsChoosingManieurMove?)
        (Variables|Default|SetIsChoosingManieurMove? false)
        (Variables|Default|SetIsChoosingAction? true)
        (Development|PrintString "return Choose Action" true true "(R=1.000000,G=0.000000,B=0.003617,A=1.000000)")))))

(event Input|EnhancedActionEvents|EnhancedInputActionIA_Y_InBattle
  (params (ActionValue :type Boolean) (ElapsedSeconds :type Float%20%28double-precision%29) (TriggeredSeconds :type Float%20%28double-precision%29) (InputAction :type Input%20Action%20Object%20Reference :default "/Game/GAME/INPUT/Actions/InBattle/IA_Y_InBattle.IA_Y_InBattle"))
  (:Started
    (if (Variables|Default|GetIsChoosingAction?)
      (Variables|Default|SetIsChoosingAction? false)
      (Variables|Default|SetIsChoosingArmeMove? true)
      (if (Variables|/Game/GAME/BP/Components/BPC_PlayableCharacter.BPC_PlayableCharacter_C|GetIsManieur? (Variables|/Game/GAME/BP/InBattle/Manieur_Armes/BP_PlayableCharacterInBattle.BP_PlayableCharacterInBattle_C|GetBPC_PlayableCharacter (Variables|Default|GetCurrentCharacter)))
        (Variables|Default|SetCurrentCharacter (Variables|/Game/GAME/BP/Components/BPC_PlayableCharacter.BPC_PlayableCharacter_C|GetAlly%20Arme%20/%20Manieur (Variables|/Game/GAME/BP/InBattle/Manieur_Armes/BP_PlayableCharacterInBattle.BP_PlayableCharacterInBattle_C|GetBPC_PlayableCharacter (Variables|Default|GetCurrentCharacter)))))
      (Development|PrintString "choose Manieur Move" true true "(R=0.000000,G=0.453341,B=1.000000,A=1.000000)")
      (elif (Variables|Default|GetIsChoosingArmeMove?)
        (Variables|Default|SetIsChoosingArmeMove? false)
        (Variables|Default|SetIsChoosingAction? true)
        (Development|PrintString "return Choose Action" true true "(R=1.000000,G=0.000000,B=0.031497,A=1.000000)")))))

(event Input|EnhancedActionEvents|EnhancedInputActionIA_A_InBattle
  (params (ActionValue :type Boolean) (ElapsedSeconds :type Float%20%28double-precision%29) (TriggeredSeconds :type Float%20%28double-precision%29) (InputAction :type Input%20Action%20Object%20Reference :default "/Game/GAME/INPUT/Actions/InBattle/IA_A_InBattle.IA_A_InBattle"))
  (bind _currentcharacter (Variables|Default|GetCurrentCharacter))
  (:Started
    (if (Variables|Default|GetIsChoosingAction?)
      (Variables|Default|SetIsChoosingAction? false)
      (Variables|Default|SetIsChoosingItem? true)
      (Development|PrintString "choose Item" true true "(R=0.065775,G=1.000000,B=0.000000,A=1.000000)")
      (elif (Variables|Default|GetIsChoosingItem?)
        (Variables|Default|SetIsChoosingAction? true)
        (Variables|Default|SetIsChoosingItem? false)
        (Development|PrintString "return Choose Action" true true "(R=1.000000,G=0.000000,B=0.031497,A=1.000000)")
        (elif (or (Variables|Default|GetIsChoosingManieurMove?) (Variables|Default|GetIsChoosingArmeMove?))
          (Default|UsePlayableCharacterMove (Variables|Default|GetGM%20ref) (Utilities|Array|Get(acopy) (Variables|/Game/GAME/BP/Components/BPC_PlayableCharacter.BPC_PlayableCharacter_C|GetUsable%20Moves (Variables|/Game/GAME/BP/InBattle/Manieur_Armes/BP_PlayableCharacterInBattle.BP_PlayableCharacterInBattle_C|GetBPC_PlayableCharacter _currentcharacter)) (Variables|Default|GetMenuIndex)) _currentcharacter))))))

(event EventBeginPlay
  (bind _asplayer_controller (Utilities|Casting|CastToPlayerController (Pawn|GetController)))
  (Utilities|IsValid (PlayerController|LocalPlayerSubsystems|GetEnhancedInputLocalPlayerSubsystem _asplayer_controller)
    (:Is%20Valid
      (Input|AddMappingContext (PlayerController|LocalPlayerSubsystems|GetEnhancedInputLocalPlayerSubsystem _asplayer_controller) "/Game/GAME/INPUT/IMC_InBattle.IMC_InBattle" 0 "(bIgnoreAllPressedKeysUntilRelease=True,bForceImmediately=False,bNotifyUserSettings=False)")
      (bind _outactors (Actor|GetAllActorsOfClass "/Game/GAME/BP/General/GM_BattleGameMode.GM_BattleGameMode_C"))
      (Variables|Default|SetGM%20ref (Utilities|Array|Get(acopy) _outactors))
      (bind _returnvalue (UserInterface|CreateWidget "/Game/GAME/BP/Widget/WBP_BattleHud.WBP_BattleHud_C"))
      (UserInterface|Viewport|AddtoViewport _returnvalue 0)
      (Utilities|FlowControl|Delay 0.1)
      (Variables|Default|SetCurrentCharacter (Utilities|Array|Get(acopy) (Variables|/Game/GAME/BP/General/GM_BattleGameMode.GM_BattleGameMode_C|GetPlayableCharacterBP_Refs (Variables|Default|GetGM%20ref)))))))

(event EventTick
  (params (DeltaSeconds :type Float%20%28single-precision%29)))

(event Collision|EventActorBeginOverlap
  (params (OtherActor :type Actor%20Object%20Reference)))

(fn ConstructionScript)