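; Playable character actor used in battle, handling facing and death for itself and its linked AllyArmeManieur partner.
; FaceTowardsOpponent turns its skeletal mesh, and the partner's if valid, by yaw only toward a given location.
; Dies prints a debug message, cascades to the partner when this character is the Manieur, then hides it, removes it from GMBattle's character list and clears IsAlive.
; AnimMagic is an empty stub.
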(event Custom|FaceTowardsOpponent
  (params (Location :type Vector))
  (bind _returnvalue (Transformation|GetActorLocation))
  (bind _bpc_playablecharacter (Variables|Default|GetBPC_PlayableCharacter))
  (bind _returnvalue_2 (Math|Rotator|FindLookatRotation _returnvalue Location))
  (bind _ally_arme___manieur (Variables|/Game/GAME/BP/Components_Interfaces/BPC_PlayableCharacter.BPC_PlayableCharacter_C|GetAlly%20Arme%20/%20Manieur _bpc_playablecharacter))
  (Transformation|SetRelativeRotation (Variables|Default|GetSkeletalMesh) (Math|Rotator|MakeRotator 0.0 0.0 (.yaw _returnvalue_2)) false false)
  (Utilities|IsValid _ally_arme___manieur
    (:Is%20Valid
      (Transformation|SetRelativeRotation (Variables|BP_PlayableCharacterInBattle_C|GetSkeletalMesh _ally_arme___manieur) (Math|Rotator|MakeRotator 0.0 0.0 (.yaw _returnvalue_2)) false false))))

(event Custom|Dies
  (bind _bpc_playablecharacter (Variables|Default|GetBPC_PlayableCharacter))
  (bind _bpc_commonstats (Variables|Default|GetBPC_CommonStats))
  (bind _ally_arme___manieur (Variables|/Game/GAME/BP/Components_Interfaces/BPC_PlayableCharacter.BPC_PlayableCharacter_C|GetAlly%20Arme%20/%20Manieur _bpc_playablecharacter))
  (Development|PrintString (Utilities|String|Append (Utilities|GetDisplayName self) " je meurt"))
  (if (Variables|/Game/GAME/BP/Components_Interfaces/BPC_PlayableCharacter.BPC_PlayableCharacter_C|GetIsManieur? _bpc_playablecharacter)
    (Utilities|IsValid _ally_arme___manieur
      (:Is%20Valid
        (CallFunction|Dies _ally_arme___manieur))
      (:Is%20Not%20Valid
        _)))
  (Rendering|SetActorHiddenInGame true)
  (Utilities|Array|RemoveItem (Variables|/Game/GAME/BP/General/GM_BattleGameMode.GM_BattleGameMode_C|GetPlayableCharacterBP_Refs (Variables|/Game/GAME/BP/Components_Interfaces/BPC_CommonStats.BPC_CommonStats_C|GetGM_Battle _bpc_commonstats)) self)
  (Variables|/Game/GAME/BP/Components_Interfaces/BPC_CommonStats.BPC_CommonStats_C|SetIsAlive? _bpc_commonstats false))

(event EventBeginPlay)

(event Collision|EventActorBeginOverlap
  (params (OtherActor :type Actor%20Object%20Reference)))

(event EventTick
  (params (DeltaSeconds :type Float%20%28single-precision%29)))

(fn ConstructionScript)

(fn AnimMagic)