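; BP_Bourrasque2 is a battle projectile actor for a gust effect, driven by its BPC_Projectile component.
; One second after that component activates, it starts the Niagara effect and a timeline that moves Sphere1 by Direction times Speed each update, without sweep.
; When the sphere overlaps the actor owning the target BPC_CommonStats, it calls CallHitEnnemy and destroys itself two seconds later.
; Overlaps while activated also print debug names.
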(event OnComponentActivated(BPC_Projectile)
  (params (Component :type Actor%20Component%20Object%20Reference) (bReset :type Boolean))
  (bind _sphere1 (Variables|Default|GetSphere1))
  (bind _bpc_projectile (Variables|Default|GetBPC_Projectile))
  (Utilities|FlowControl|Delay 1.0)
  (Components|Activation|Activate (Variables|Default|GetNS_Bourrasque1) true)
  (Timeline|Timeline PlayFromStart
    (:Update
      (Transformation|SetWorldLocation _sphere1 (+ (Transformation|GetWorldLocation _sphere1) (* (Variables|/Game/GAME/BP/Components_Interfaces/BPC_Projectile.BPC_Projectile_C|GetDirection _bpc_projectile) (Variables|/Game/GAME/BP/Components_Interfaces/BPC_Projectile.BPC_Projectile_C|GetSpeed _bpc_projectile))) false false))))

(event OnComponentBeginOverlap(Sphere1)
  (params (OverlappedComponent :type Primitive%20Component%20Object%20Reference) (OtherActor :type Actor%20Object%20Reference) (OtherComp :type Primitive%20Component%20Object%20Reference) (OtherBodyIndex :type Integer) (bFromSweep :type Boolean) (SweepResult :type Hit%20Result%20Structure%20%28by%20ref%29))
  (bind _bpc_projectile (Variables|Default|GetBPC_Projectile))
  (bind _bpc_target (Variables|/Game/GAME/BP/Components_Interfaces/BPC_Projectile.BPC_Projectile_C|GetBPC_Target _bpc_projectile))
  (if (Variables|/Game/GAME/BP/Components_Interfaces/BPC_Projectile.BPC_Projectile_C|GetActivated (Variables|Default|GetBPC_Projectile))
    (Development|PrintString (Utilities|String|Append (Utilities|GetDisplayName _bpc_target) " : " (Utilities|GetDisplayName OtherActor)))
    (if (== (Actor|GetComponentbyClass OtherActor "/Game/GAME/BP/Components_Interfaces/BPC_CommonStats.BPC_CommonStats_C") _bpc_target)
      (Default|CallHitEnnemy (Variables|Default|GetBPC_Projectile))
      (Utilities|FlowControl|Delay 2.0)
      (Actor|DestroyActor))))

(event EventBeginPlay
  (|CallParentFunction) ; This node is disabled and will not be called.\nDrag off pins to build functionality.
)

(event Collision|EventActorBeginOverlap
  (params (OtherActor :type Actor%20Object%20Reference))
  (|CallParentFunction OtherActor) ; This node is disabled and will not be called.\nDrag off pins to build functionality.
)

(fn ConstructionScript
  (|CallParentFunction))