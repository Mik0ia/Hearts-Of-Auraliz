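; Water bubble projectile for battle that flies along a set direction and hits one designated target.
; When BPC_Projectile activates, it starts the bubble effect and a Timeline that moves the scene root by Direction times Speed each update, without delta-time scaling.
; A sphere overlap matching the target's BPC_CommonStats reports the hit, stops movement, swaps bubbles for a splash effect and destroys the actor after a delay.
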(event OnComponentActivated(BPC_Projectile)
  (params (Component :type Actor%20Component%20Object%20Reference) (bReset :type Boolean))
  (bind _scene (Variables|Default|GetScene))
  (bind _bpc_projectile (Variables|Default|GetBPC_Projectile))
  (Components|Activation|Activate (Variables|Default|GetNS_Magic_Big_Bubbles_Owner_Cast1) true)
  (Timeline|Timeline PlayFromStart
    (:Update
      (Transformation|SetWorldLocation _scene (+ (Transformation|GetWorldLocation _scene) (* (Variables|/Game/GAME/BP/Components_Interfaces/BPC_Projectile.BPC_Projectile_C|GetDirection _bpc_projectile) (Variables|/Game/GAME/BP/Components_Interfaces/BPC_Projectile.BPC_Projectile_C|GetSpeed _bpc_projectile))) false false))))

(event OnComponentBeginOverlap(Sphere)
  (params (OverlappedComponent :type Primitive%20Component%20Object%20Reference) (OtherActor :type Actor%20Object%20Reference) (OtherComp :type Primitive%20Component%20Object%20Reference) (OtherBodyIndex :type Integer) (bFromSweep :type Boolean) (SweepResult :type Hit%20Result%20Structure%20%28by%20ref%29))
  (bind _scene (Variables|Default|GetScene))
  (bind _bpc_projectile (Variables|Default|GetBPC_Projectile))
  (bind _bpc_projectile_2 (Variables|Default|GetBPC_Projectile))
  (bind _bpc_target (Variables|/Game/GAME/BP/Components_Interfaces/BPC_Projectile.BPC_Projectile_C|GetBPC_Target _bpc_projectile_2))
  (if (Variables|/Game/GAME/BP/Components_Interfaces/BPC_Projectile.BPC_Projectile_C|GetActivated (Variables|Default|GetBPC_Projectile))
    (Development|PrintString (Utilities|String|Append (Utilities|GetDisplayName _bpc_target) " : " (Utilities|GetDisplayName OverlappedComponent)))
    (if (== (Actor|GetComponentbyClass OtherActor "/Game/GAME/BP/Components_Interfaces/BPC_CommonStats.BPC_CommonStats_C") _bpc_target)
      (Utilities|FlowControl|Sequence
        (:then_0
          (Default|CallHitEnnemy (Variables|Default|GetBPC_Projectile))
          (Development|SetHiddeninGame (Variables|Default|GetNS_Magic_Big_Bubbles_Owner_Cast1) true false)
          (Variables|/Game/GAME/BP/Components_Interfaces/BPC_Projectile.BPC_Projectile_C|SetActivated (Variables|Default|GetBPC_Projectile) false)
          (Components|Activation|Activate (Variables|Default|GetP_ky_waterBallHit) false)
          (Utilities|FlowControl|Delay 3.0)
          (Actor|DestroyActor))
        (:then_1
          (Timeline|Timeline Stop
            (:Update
              (Transformation|SetWorldLocation _scene (+ (Transformation|GetWorldLocation _scene) (* (Variables|/Game/GAME/BP/Components_Interfaces/BPC_Projectile.BPC_Projectile_C|GetDirection _bpc_projectile) (Variables|/Game/GAME/BP/Components_Interfaces/BPC_Projectile.BPC_Projectile_C|GetSpeed _bpc_projectile))) false false))))))))

(event EventBeginPlay
  (|CallParentFunction)
  (Development|PrintString "j'ai spawn"))

(event Collision|EventActorBeginOverlap
  (params (OtherActor :type Actor%20Object%20Reference))
  (|CallParentFunction OtherActor) ; This node is disabled and will not be called.\nDrag off pins to build functionality.
)

(event EventTick
  (params (DeltaSeconds :type Float%20%28single-precision%29))
  (|CallParentFunction DeltaSeconds) ; This node is disabled and will not be called.\nDrag off pins to build functionality.
)

(fn ConstructionScript
  (|CallParentFunction))