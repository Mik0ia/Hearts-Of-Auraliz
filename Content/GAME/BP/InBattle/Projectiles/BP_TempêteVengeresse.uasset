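; BP_TempêteVengeresse is an in-battle projectile Blueprint for the Tempête Vengeresse attack, which strikes directly at its target's position.
; When its projectile component activates, it teleports onto the target's owner actor without sweeping and activates area and slash Niagara effects.
; After a short delay, a DoOnce-guarded step triggers the component's enemy hit, then the actor destroys itself once a longer delay elapses.
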(event OnComponentActivated(BPC_Projectile)
  (params (Component :type Actor%20Component%20Object%20Reference) (bReset :type Boolean))
  (Transformation|SetActorLocation (Transformation|GetActorLocation (Components|GetOwner (Variables|/Game/GAME/BP/Components_Interfaces/BPC_Projectile.BPC_Projectile_C|GetBPC_Target (Variables|Default|GetBPC_Projectile)))) false false)
  (Components|Activation|Activate (Variables|Default|GetNS_Free_Magic_Area2) true)
  (Components|Activation|Activate (Variables|Default|GetNS_Free_Magic_Slash) true)
  (Utilities|FlowControl|Delay 0.5)
  (Utilities|FlowControl|DoOnce false
    (:Completed
      (Default|CallHitEnnemy (Variables|Default|GetBPC_Projectile))
      (Utilities|FlowControl|Delay 6.0)
      (Actor|DestroyActor))))

(event EventBeginPlay
  (|CallParentFunction))

(event Collision|EventActorBeginOverlap
  (params (OtherActor :type Actor%20Object%20Reference))
  (|CallParentFunction OtherActor) ; This node is disabled and will not be called.\nDrag off pins to build functionality.
)

(event EventTick
  (params (DeltaSeconds :type Float%20%28single-precision%29))
  (|CallParentFunction DeltaSeconds) ; This node is disabled and will not be called.\nDrag off pins to build functionality.
)

(fn ConstructionScript
  (|CallParentFunction))