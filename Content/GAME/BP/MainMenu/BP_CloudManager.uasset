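; Main menu cloud manager that fills its Box volume with BP_MovingCloud actors on BeginPlay, up to MaxCloudsNumbers.
; Initial clouds get random position, yaw, scale and a HeterogeneousVolume material picked from MaterialsList, with an index range that overruns the array.
; DestroyRespawnCloud recycles a given cloud by destroying it and spawning a randomly scaled replacement inside CloudStartRef's box.
; Replacements keep their default material because that SetMaterial step is unconnected.
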(event Collision|EventActorBeginOverlap
  (params (OtherActor :type Actor%20Object%20Reference)))

(event EventBeginPlay
  (Utilities|SpawnNumberOfClouds (Variables|Default|GetMax%20Clouds%20Numbers)))

(fn ConstructionScript)

(fn SpawnCloud
  (bind _box (Variables|Default|GetBox))
  (bind _materialslist (Variables|Default|GetMaterialsList))
  (bind _returnvalue (Game|SpawnActorfromClass "/Game/GAME/BP/MainMenu/BP_MovingCloud.BP_MovingCloud_C" (Math|Transform|MakeTransform (Math|Random|RandomPointinBoundingBox (Transformation|GetWorldLocation _box) (Variables|/Script/Engine.BoxComponent|GetBoxExtent _box)) (Math|Rotator|MakeRotator 0.0 0.0 (Math|Random|RandomFloatinRange 0.0 1.8e+02)) (* (Math|Vector|MakeVector 1.0 1.0 1.0) (Math|Random|RandomFloatinRange 1e+01 15.0))) "AlwaysSpawn" "MultiplyWithRoot" 0 0))
  (Rendering|Material|SetMaterial (Variables|/Game/GAME/BP/MainMenu/BP_MovingCloud.BP_MovingCloud_C|GetHeterogeneousVolume _returnvalue) 0 (Utilities|Array|Get(acopy) _materialslist (Math|Random|RandomIntegerinRange 0 (+ (Utilities|Array|Length _materialslist) 1)))))

(fn SpawnCloudatStart
  (bind _cloudstartref (Variables|Default|GetCloudStartRef))
  (bind _box (Variables|/Game/GAME/BP/MainMenu/BP_CloudStart.BP_CloudStart_C|GetBox _cloudstartref))
  (bind _returnvalue (Game|SpawnActorfromClass "/Game/GAME/BP/MainMenu/BP_MovingCloud.BP_MovingCloud_C" (Math|Transform|MakeTransform (Math|Random|RandomPointinBoundingBox (Transformation|GetWorldLocation _box) (Variables|/Script/Engine.BoxComponent|GetBoxExtent _box)) "0, 0, 0" (* (Math|Vector|MakeVector 1.0 1.0 1.0) (Math|Random|RandomFloatinRange 1e+01 15.0))) "AlwaysSpawn" "MultiplyWithRoot" 0 0)))

(fn Destroy+RespawnCloud
  (params (Cloud%20Ref :type BP%20Moving%20Cloud%20Object%20Reference))
  (Actor|DestroyActor Cloud%20Ref)
  (CallFunction|SpawnCloudatStart))