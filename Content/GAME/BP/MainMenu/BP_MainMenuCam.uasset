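; BP_MainMenuCam is the main menu actor that brings up the menu and handles its press-a-key screen.
; On BeginPlay it shows WBP_MainMenu, plays the Call_Of_Auraliz sound, then enables the mouse cursor and adds the IMC_Main_Menu Enhanced Input context through its player controller.
; The IA_PressAKey action tells the widget to go to the main menu, with a flag preventing repeat transitions.
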(event Input|EnhancedActionEvents|EnhancedInputActionIA_PressAKey
  (params (ActionValue :type Boolean) (ElapsedSeconds :type Float%20%28double-precision%29) (TriggeredSeconds :type Float%20%28double-precision%29) (InputAction :type Input%20Action%20Object%20Reference :default "/Game/GAME/INPUT/IA_PressAKey.IA_PressAKey"))
  (:Started
    (if (Variables|Default|GetIsInPressAKeyMenu)
      (Default|GotoMainMenu (Variables|Default|GetWidgetMenu))
      (Variables|Default|SetIsInPressAKeyMenu false))))

(event EventBeginPlay
  (bind _returnvalue (UserInterface|CreateWidget "/Game/GAME/BP/MainMenu/WBP_MainMenu.WBP_MainMenu_C"))
  (bind _output_get (Variables|Default|SetWidgetMenu _returnvalue))
  (UserInterface|Viewport|AddtoViewport _output_get 0)
  (Audio|PlaySound2D "/Game/GAME/AUDIO/MUSIC/Call_Of_Auraliz.Call_Of_Auraliz" 1.0 1.0 0.0 0 0)
  (bind _asplayer_controller (Utilities|Casting|CastToPlayerController (Pawn|GetController)))
  (Variables|/Script/Engine.PlayerController|SetbShowMouseCursor _asplayer_controller true)
  (Utilities|IsValid (PlayerController|LocalPlayerSubsystems|GetEnhancedInputLocalPlayerSubsystem _asplayer_controller)
    (:Is%20Valid
      (Input|AddMappingContext (PlayerController|LocalPlayerSubsystems|GetEnhancedInputLocalPlayerSubsystem _asplayer_controller) "/Game/GAME/INPUT/IMC_Main_Menu.IMC_Main_Menu" 0 "(bIgnoreAllPressedKeysUntilRelease=True,bForceImmediately=False,bNotifyUserSettings=False)"))))

(fn ConstructionScript)