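; BP_CampFire is an overworld campfire that the player interacts with to open a dialogue from DT_Firecamp.
; While active, interaction registers it as the game mode's current campfire and saves the player's location to the game instance as the last campfire coordinate.
; Deactivate turns off fire and smoke effects and starts a cooldown.
; Tick uses a DoOnce-gated one-second delay to count to sixty, printing progress, then reactivates it.
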(event OnComponentActivated(BPC_Interactable)
  (params (Component :type Actor%20Component%20Object%20Reference) (bReset :type Boolean))
  (if (Variables|Default|GetIsActive?)
    (bind _output_get (Variables|Default|SetPlayer (Variables|/Game/GAME/BP/Components_Interfaces/BPC_Interactable.BPC_Interactable_C|GetPlayer (Variables|Default|GetBPC_Interactable))))
    (CallFunction|AskifWanttoUseFirecamp? _output_get)))

(event Custom|AskIf%20WantToUseFirecamp?
  (params (Player :type BP%20Player%20Character%20Object%20Reference))
  (bind _bpc_dialogue (Variables|Default|GetBPC_Dialogue))
  (bind _output_get (Variables|/Game/GAME/BP/Components_Interfaces/BPC_Dialogue.BPC_Dialogue_C|SetPlayer _bpc_dialogue Player))
  (Variables|/Game/GAME/BP/General/GM_OverworldGameMode.GM_OverworldGameMode_C|SetCurrentFirecamp (Variables|/Game/GAME/BP/Overworld/BP_PlayerCharacter.BP_PlayerCharacter_C|GetGM%20Ref _output_get) self)
  (Variables|/Game/GAME/BP/General/GI_GameInstance.GI_GameInstance_C|SetLastCampfireCoord (Variables|/Game/GAME/BP/General/GM_OverworldGameMode.GM_OverworldGameMode_C|GetAs%20GI%20Game%20Instance (Variables|/Game/GAME/BP/Overworld/BP_PlayerCharacter.BP_PlayerCharacter_C|GetGM%20Ref _output_get)) (Transformation|GetActorLocation Player))
  (Default|LaunchDialogue _bpc_dialogue "/Game/GAME/DATA/DATA_TABLE/Dialogues/DT_Firecamp.DT_Firecamp" 1))

(event Custom|Deactivate
  (Components|Activation|Deactivate (Variables|Default|GetNiagara))
  (Components|Activation|Deactivate (Variables|Default|GetP_Smoke))
  (Variables|Default|SetCurrentValue 0.0)
  (Variables|Default|SetIsActive? false)
  (Variables|Default|SetIsInCooldown true))

(event Custom|Activate
  (Components|Activation|Activate (Variables|Default|GetNiagara) false)
  (Components|Activation|Activate (Variables|Default|GetP_Smoke) true)
  (Variables|Default|SetCurrentValue 0.0)
  (Variables|Default|SetIsActive? true)
  (Variables|Default|SetIsInCooldown false))

(event EventTick
  (params (DeltaSeconds :type Float%20%28single-precision%29))
  (if (Variables|Default|GetIsInCooldown)
    (Utilities|FlowControl|DoOnce false :!label _label
      (:Completed
        (Utilities|FlowControl|Delay 1.0)
        (bind _output_get (Variables|Default|SetCurrentValue (+ (Variables|Default|GetCurrentValue) 1.0)))
        (Development|PrintString (Utilities|String|ToString(Float) _output_get))
        (if (>= _output_get 6e+01)
          (CallFunction|Activate)
          (goto _label Reset)
          (else
            (goto _label Reset)))))))

(fn ConstructionScript)