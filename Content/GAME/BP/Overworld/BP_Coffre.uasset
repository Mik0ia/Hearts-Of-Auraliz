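; BP_Coffre is an interactable overworld chest whose lid swings open and shut when its BPC_Interactable component activates.
; It disables the interacting player's input, then a timeline rolls the CoffreHaut lid open from its current relative rotation.
; After a short delay, a second timeline rolls the lid back and re-enables input when finished.
; The graph handles only this animation and input lock, with no reward logic.
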(event OnComponentActivated(BPC_Interactable)
  (params (Component :type Actor%20Component%20Object%20Reference) (bReset :type Boolean))
  (bind _coffre_haut (Variables|Default|GetCoffre_Haut))
  (bind _coffre_haut_2 (Variables|Default|GetCoffre_Haut))
  (bind _bpc_interactable (Variables|Default|GetBPC_Interactable))
  (bind _player (Variables|/Game/GAME/BP/Components_Interfaces/BPC_Interactable.BPC_Interactable_C|GetPlayer _bpc_interactable))
  (Input|DisableInput _player 0)
  (Variables|Default|SetTempRot (Variables|/Script/Engine.SceneComponent|GetRelativeRotation _coffre_haut))
  (bind _newtrack_0 (Timeline|Timeline PlayFromStart)
    (:Update
      (Transformation|SetRelativeRotation _coffre_haut (Math|Rotator|Lerp(Rotator) (Variables|/Script/Engine.SceneComponent|GetRelativeRotation _coffre_haut) (Math|Rotator|MakeRotator (+ (.roll (Variables|Default|GetTempRot)) 4e+01) (.pitch (Variables|Default|GetTempRot)) (.yaw (Variables|Default|GetTempRot))) _newtrack_0) false false))
    (:Finished
      (Utilities|FlowControl|Delay 1.0)
      (Variables|Default|SetTempRot (Variables|/Script/Engine.SceneComponent|GetRelativeRotation _coffre_haut_2))
      (bind _newtrack_0_2 (Timeline|Timeline_0 PlayFromStart)
        (:Update
          (Transformation|SetRelativeRotation _coffre_haut_2 (Math|Rotator|Lerp(Rotator) (Variables|/Script/Engine.SceneComponent|GetRelativeRotation _coffre_haut_2) (Math|Rotator|MakeRotator (+ (.roll (Variables|Default|GetTempRot)) -4e+01) (.pitch (Variables|Default|GetTempRot)) (.yaw (Variables|Default|GetTempRot))) _newtrack_0_2) false false))
        (:Finished
          (Input|EnableInput _player 0))))))

(event EventBeginPlay)

(event Collision|EventActorBeginOverlap
  (params (OtherActor :type Actor%20Object%20Reference)))

(event EventTick
  (params (DeltaSeconds :type Float%20%28single-precision%29)))

(fn ConstructionScript)