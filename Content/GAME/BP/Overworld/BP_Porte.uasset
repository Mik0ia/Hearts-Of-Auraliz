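; Overworld door that, when activated through its interactable component, teleports the player to a linked door.
; A timeline swings the door mesh slightly open with collision disabled while player input is locked.
; A fade widget then covers the move to the AimingDoor's TPRoot transform, during which the door's rotation is zeroed and its collision restored.
; The fade plays in reverse before input returns and the widget is removed.
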(event OnComponentActivated(BPC_Interactable)
  (params (Component :type Actor%20Component%20Object%20Reference) (bReset :type Boolean))
  (bind _aiming_door (Variables|Default|GetAiming%20Door))
  (bind _sm_door2 (Variables|Default|GetSM_Door2))
  (bind _sm_door2_2 (Variables|Default|GetSM_Door2))
  (bind _bpc_interactable (Variables|Default|GetBPC_Interactable))
  (bind _tp_root (Variables|BP_Porte_C|GetTP_Root _aiming_door))
  (bind _player (Variables|/Game/GAME/BP/Components_Interfaces/BPC_Interactable.BPC_Interactable_C|GetPlayer _bpc_interactable))
  (Input|DisableInput _player 0)
  (Collision|SetCollisionEnabled (Variables|Default|GetSM_Door2) "NoCollision")
  (Variables|Default|SetTempRot (Variables|/Script/Engine.SceneComponent|GetRelativeRotation _sm_door2_2))
  (bind _newtrack_0 (Timeline|Timeline PlayFromStart)
    (:Update
      (Transformation|SetRelativeRotation _sm_door2_2 (Math|Rotator|Lerp(Rotator) (Variables|/Script/Engine.SceneComponent|GetRelativeRotation _sm_door2_2) (Math|Rotator|MakeRotator (.roll (Variables|Default|GetTempRot)) (.pitch (Variables|Default|GetTempRot)) (- (.yaw (Variables|Default|GetTempRot)) 15.0)) _newtrack_0) false false))
    (:Finished
      (bind _returnvalue (UserInterface|CreateWidget "/Game/GAME/BP/Widget/WBP_Fade.WBP_Fade_C"))
      (UserInterface|Viewport|AddtoViewport _returnvalue 0)
      (Utilities|FlowControl|Delay 1.0)
      (Transformation|SetActorTransform _player (Math|Transform|MakeTransform (Transformation|GetWorldLocation _tp_root) (Transformation|GetWorldRotation _tp_root) "1.000000,1.000000,1.000000"))
      (Transformation|SetRelativeRotation _sm_door2 "0, 0, 0" false false)
      (Collision|SetCollisionEnabled _sm_door2 "QueryAndPhysics")
      (Utilities|FlowControl|Delay 1.0)
      (Class|UserWidget|PlayAnimationReverse _returnvalue (Variables|/Game/GAME/BP/Widget/WBP_Fade.WBP_Fade_C|GetFadeIn _returnvalue) 1.0 false)
      (Utilities|FlowControl|Delay 1.0)
      (Input|EnableInput _player 0)
      (Widget|RemovefromParent _returnvalue))))

(fn ConstructionScript)