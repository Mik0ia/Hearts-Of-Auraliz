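; Overworld road trigger actor that starts a directional road dialogue when the player enters either of its two boxes.
; Each box stores its arrow's forward vector on the player, then launches BPCDialogue with the same DT_RoadDialogue entry.
; An IsActive flag and DoOnce nodes gate the triggers; Resolve re-arms both boxes and sets IsActive.
; A middle sphere calls MiddleOfRoadEvent on the player's GMRef once, without being re-armed.
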(event OnComponentBeginOverlap(Sphere)
  (params (OverlappedComponent :type Primitive%20Component%20Object%20Reference) (OtherActor :type Actor%20Object%20Reference) (OtherComp :type Primitive%20Component%20Object%20Reference) (OtherBodyIndex :type Integer) (bFromSweep :type Boolean) (SweepResult :type Hit%20Result%20Structure%20%28by%20ref%29))
  (if (Variables|Default|GetIsActive?)
    (Utilities|IsValid (Actor|GetComponentbyClass OtherActor "/Game/GAME/BP/Components_Interfaces/BPC_PlayerOverworld.BPC_PlayerOverworld_C")
      (:Is%20Valid
        (Utilities|FlowControl|DoOnce false
          (:Completed
            (bind _asbp_player_character (Utilities|Casting|CastToBP_PlayerCharacter OtherActor))
            (bind _output_get (Variables|Default|SetAs%20BP%20Player%20Character _asbp_player_character))
            (Default|MiddleOfRoadEvent (Variables|/Game/GAME/BP/Overworld/BP_PlayerCharacter.BP_PlayerCharacter_C|GetGM%20Ref _output_get))))))))

(event OnComponentBeginOverlap(Box)
  (params (OverlappedComponent :type Primitive%20Component%20Object%20Reference) (OtherActor :type Actor%20Object%20Reference) (OtherComp :type Primitive%20Component%20Object%20Reference) (OtherBodyIndex :type Integer) (bFromSweep :type Boolean) (SweepResult :type Hit%20Result%20Structure%20%28by%20ref%29))
  (bind _bpc_dialogue (Variables|Default|GetBPC_Dialogue))
  (if (Variables|Default|GetIsActive?)
    (Utilities|IsValid (Actor|GetComponentbyClass OtherActor "/Game/GAME/BP/Components_Interfaces/BPC_PlayerOverworld.BPC_PlayerOverworld_C")
      (:Is%20Valid
        (Utilities|FlowControl|DoOnce false
          (:Completed
            (bind _asbp_player_character (Utilities|Casting|CastToBP_PlayerCharacter OtherActor))
            (bind _output_get (Variables|Default|SetAs%20BP%20Player%20Character _asbp_player_character))
            (Variables|/Game/GAME/BP/Overworld/BP_PlayerCharacter.BP_PlayerCharacter_C|SetCurrentDirectionRoadDialogue _output_get (Math|Vector|GetForwardVector (Variables|Default|GetArrow1)))
            (Variables|/Game/GAME/BP/Components_Interfaces/BPC_Dialogue.BPC_Dialogue_C|SetPlayer _bpc_dialogue _output_get)
            (Default|LaunchDialogue _bpc_dialogue "/Game/GAME/DATA/DATA_TABLE/Dialogues/Wild_Island/DT_RoadDialogue.DT_RoadDialogue" 1)))))))

(event OnComponentBeginOverlap(Box1)
  (params (OverlappedComponent :type Primitive%20Component%20Object%20Reference) (OtherActor :type Actor%20Object%20Reference) (OtherComp :type Primitive%20Component%20Object%20Reference) (OtherBodyIndex :type Integer) (bFromSweep :type Boolean) (SweepResult :type Hit%20Result%20Structure%20%28by%20ref%29))
  (bind _bpc_dialogue (Variables|Default|GetBPC_Dialogue))
  (if (Variables|Default|GetIsActive?)
    (Utilities|IsValid (Actor|GetComponentbyClass OtherActor "/Game/GAME/BP/Components_Interfaces/BPC_PlayerOverworld.BPC_PlayerOverworld_C")
      (:Is%20Valid
        (Utilities|FlowControl|DoOnce false
          (:Completed
            (bind _asbp_player_character (Utilities|Casting|CastToBP_PlayerCharacter OtherActor))
            (bind _output_get (Variables|Default|SetAs%20BP%20Player%20Character _asbp_player_character))
            (Variables|/Game/GAME/BP/Overworld/BP_PlayerCharacter.BP_PlayerCharacter_C|SetCurrentDirectionRoadDialogue _output_get (Math|Vector|GetForwardVector (Variables|Default|GetArrow)))
            (Variables|/Game/GAME/BP/Components_Interfaces/BPC_Dialogue.BPC_Dialogue_C|SetPlayer _bpc_dialogue _output_get)
            (Default|LaunchDialogue _bpc_dialogue "/Game/GAME/DATA/DATA_TABLE/Dialogues/Wild_Island/DT_RoadDialogue.DT_RoadDialogue" 1)))))))

(event Custom|Resolve
  (bind _bpc_dialogue (Variables|Default|GetBPC_Dialogue))
  (bind _bpc_dialogue_2 (Variables|Default|GetBPC_Dialogue))
  (Utilities|FlowControl|Sequence
    (:then_0
      (Utilities|FlowControl|DoOnce false) ; enters at Reset
    )
    (:then_1
      (Utilities|FlowControl|DoOnce false) ; enters at Reset
    )
    (:then_2
      (Variables|Default|SetIsActive? true))))

(fn ConstructionScript)