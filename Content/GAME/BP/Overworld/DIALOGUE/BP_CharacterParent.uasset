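; Parent Blueprint for overworld characters the player can talk to, turning the mesh during dialogue.
; Activating the interactable component saves the mesh rotation, passes the player to the dialogue component and launches the current DataTable row.
; One timeline eases mesh yaw using the player-to-character direction, while another restores the saved yaw when dialogue finishes.
; Both lerp from the live rotation each update, keeping saved pitch and roll.
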(event OnComponentActivated(BPC_Interactable)
  (params (Component :type Actor%20Component%20Object%20Reference) (bReset :type Boolean))
  (bind _bpc_dialogue (Variables|Default|GetBPC_Dialogue))
  (bind _mesh (Variables|Character|GetMesh))
  (Variables|Default|SetBasRot (Transformation|GetWorldRotation (Variables|Character|GetMesh)))
  (Variables|/Game/GAME/BP/Components_Interfaces/BPC_Dialogue.BPC_Dialogue_C|SetPlayer _bpc_dialogue (Variables|/Game/GAME/BP/Components_Interfaces/BPC_Interactable.BPC_Interactable_C|GetPlayer (Variables|Default|GetBPC_Interactable)))
  (Default|LaunchDialogue _bpc_dialogue (Variables|/Game/GAME/BP/Components_Interfaces/BPC_Dialogue.BPC_Dialogue_C|GetDialogueDataTable _bpc_dialogue) (Variables|/Game/GAME/BP/Components_Interfaces/BPC_Dialogue.BPC_Dialogue_C|GetCurrentRowIndex _bpc_dialogue))
  (bind _newtrack_0 (Timeline|Timeline PlayFromStart)
    (:Update
      (Transformation|SetWorldRotation _mesh (Math|Rotator|MakeRotator (.roll (Variables|Default|GetBasRot)) (.pitch (Variables|Default|GetBasRot)) (.yaw (Math|Rotator|Lerp(Rotator) (Transformation|GetWorldRotation _mesh) (Math|Rotator|MakeRotfromZ (- (Transformation|GetActorLocation) (Transformation|GetActorLocation (Variables|/Game/GAME/BP/Components_Interfaces/BPC_Interactable.BPC_Interactable_C|GetPlayer (Variables|Default|GetBPC_Interactable))))) _newtrack_0))) false false))))

(event FinishedDialogue(BPC_Dialogue)
  (bind _mesh (Variables|Character|GetMesh))
  (bind _basrot (Variables|Default|GetBasRot))
  (bind _newtrack_0 (Timeline|Timeline_0 PlayFromStart)
    (:Update
      (Transformation|SetWorldRotation _mesh (Math|Rotator|MakeRotator (.roll _basrot) (.pitch _basrot) (.yaw (Math|Rotator|Lerp(Rotator) (Transformation|GetWorldRotation _mesh) (Variables|Default|GetBasRot) _newtrack_0))) false false))))

(event EventBeginPlay)

(event Collision|EventActorBeginOverlap
  (params (OtherActor :type Actor%20Object%20Reference)))

(event EventTick
  (params (DeltaSeconds :type Float%20%28single-precision%29)))

(fn ConstructionScript)