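; Out-of-bounds trigger box for the overworld that returns the player to a nearby checkpoint.
; On overlap by an actor with BPC_PlayerOverworld, it disables input and plays a WBP_Fade fade-in.
; It then scans all BP_CheckPoint actors for the closest, moves the player there and reverses the fade.
; A DoOnce blocks retriggering until the fade ends and input returns, though ClosestRange is never reset between uses.
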(event OnComponentBeginOverlap(Box)
  (params (OverlappedComponent :type Primitive%20Component%20Object%20Reference) (OtherActor :type Actor%20Object%20Reference) (OtherComp :type Primitive%20Component%20Object%20Reference) (OtherBodyIndex :type Integer) (bFromSweep :type Boolean) (SweepResult :type Hit%20Result%20Structure%20%28by%20ref%29))
  (bind _returnvalue (Actor|GetComponentbyClass OtherActor "/Game/GAME/BP/Components_Interfaces/BPC_PlayerOverworld.BPC_PlayerOverworld_C"))
  (Utilities|IsValid _returnvalue
    (:Is%20Valid
      (Utilities|FlowControl|DoOnce false :!label _label
        (:Completed
          (bind _asbp_player_character (Utilities|Casting|CastToBP_PlayerCharacter (Components|GetOwner _returnvalue)))
          (bind _returnvalue_2 (UserInterface|CreateWidget "/Game/GAME/BP/Widget/WBP_Fade.WBP_Fade_C"))
          (Components|Animation|PlayAnimation _returnvalue_2 (Variables|/Game/GAME/BP/Widget/WBP_Fade.WBP_Fade_C|GetFadeIn _returnvalue_2) 0.0
            (:then
              (Input|DisableInput _asbp_player_character 0)
              (UserInterface|Viewport|AddtoViewport _returnvalue_2 0))
            (:Finished
              (bind _outactors (Actor|GetAllActorsOfClass "/Game/GAME/BP/Overworld/MANAGER/BP_CheckPoint.BP_CheckPoint_C"))
              (for _array_element _outactors
                (if (< (Math|Vector|VectorLength (- (Transformation|GetActorLocation _array_element) (Transformation|GetActorLocation _asbp_player_character))) (Variables|Default|GetClosestRange))
                  (Variables|Default|SetClosestLocation (Transformation|GetActorLocation _array_element))
                  (Variables|Default|SetClosestRange (Math|Vector|VectorLength (- (Transformation|GetActorLocation _array_element) (Transformation|GetActorLocation _asbp_player_character))))))
              (Development|PrintString (Utilities|String|ToString(Vector) (Variables|Default|GetClosestLocation)))
              (Transformation|SetActorLocation _asbp_player_character (Variables|Default|GetClosestLocation) false false)
              (Utilities|FlowControl|Delay 0.2)
              (Components|Animation|PlayAnimation _returnvalue_2 (Variables|/Game/GAME/BP/Widget/WBP_Fade.WBP_Fade_C|GetFadeIn _returnvalue_2) 0.0 1 "Reverse"
                (:Finished
                  (Input|EnableInput _asbp_player_character 0)
                  (Widget|RemovefromParent _returnvalue_2)
                  (goto _label Reset))))))))))

(event EventBeginPlay)

(event Collision|EventActorBeginOverlap
  (params (OtherActor :type Actor%20Object%20Reference)))

(event EventTick
  (params (DeltaSeconds :type Float%20%28single-precision%29)))

(fn ConstructionScript)